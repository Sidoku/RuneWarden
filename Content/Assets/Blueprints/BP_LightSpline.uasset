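; BP_LightSpline is a patrol route Blueprint that holds a spline, PatrolRoute, and a current point index.
; GetSplinePointAsWorldPosition returns the world location of the spline point at that index.
; IncrementPatrolRoute is empty: the logic to step the index and flip Direction at either end for back-and-forth movement is present but disconnected, so nothing here advances the index.
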(event Custom|IncrementPatrolRoute)

(fn ConstructionScript)

(fn GetSplinePointasWorldPosition
  (return (Spline|GetLocationatSplinePoint (Variables|Default|GetPatrolRoute) (Variables|Default|GetPatroIndex) "World")))