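; Base projectile actor for attacks that flies at a configurable speed and gravity and can home in on an attack target.
; The construction script configures ProjectileMovement and, when homing is enabled, tracks the target's root component.
; On BeginPlay it ignores collision with its owner and aims its velocity at any valid target, homing or not.
; A box collision hit dispatches OnProjectileImpact with the hit actor and result, then destroys the projectile.
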(event OnComponentHit(BoxCollision)
  (params (HitComponent :type Primitive%20Component%20Object%20Reference) (OtherActor :type Actor%20Object%20Reference) (OtherComp :type Primitive%20Component%20Object%20Reference) (NormalImpulse :type Vector :default "0, 0, 0") (Hit :type Hit%20Result%20Structure%20%28by%20ref%29))
  ;[1 1 1] Dispatch event on impact
  (Default|CallOnProjectileImpact OtherActor Hit)
  (Actor|DestroyActor))

(event Custom|RotateToTarget
  ;[1 1 1] Rotate projectile towards homing target
  (Variables|/Script/Engine.MovementComponent|SetVelocity (Variables|Default|GetProjectileMovement) (* (Math|Vector|GetUnitDirection(Vector) (Transformation|GetActorLocation) (Transformation|GetActorLocation (Variables|Target|GetAttackTarget))) (Variables|ProjectileSettings|GetSpeed))))

(event EventBeginPlay
  ;[1 1 1] Ignore the collision with spawning actor
  (Collision|IgnoreActorwhenMoving (Variables|Default|GetBoxCollision) (Components|GetOwner) true)
  ;[1 1 1] Set homing attack target and call rotate event
  (Variables|Target|GetAttackTarget
    (:then
      (CallFunction|RotatetoTarget))
    (:else)))

(fn ConstructionScript
  (bind _projectilemovement (Variables|Default|GetProjectileMovement))
  (bind _speed (Variables|ProjectileSettings|GetSpeed))
  (Variables|/Script/Engine.ProjectileMovementComponent|SetInitialSpeed _projectilemovement _speed)
  (Variables|/Script/Engine.ProjectileMovementComponent|SetMaxSpeed _projectilemovement _speed)
  (Variables|/Script/Engine.ProjectileMovementComponent|SetProjectileGravityScale _projectilemovement (Variables|ProjectileSettings|GetGravity))
  (Variables|Target|GetAttackTarget
    (:then
      (if (Variables|ProjectileSettings|GetIsHoming)
        (Variables|/Script/Engine.ProjectileMovementComponent|SetbIsHomingProjectile _projectilemovement true)
        (Variables|/Script/Engine.ProjectileMovementComponent|SetHomingTargetComponent _projectilemovement (Variables|/Script/Engine.Actor|GetRootComponent (Variables|Target|GetAttackTarget)))))
    (:else)))