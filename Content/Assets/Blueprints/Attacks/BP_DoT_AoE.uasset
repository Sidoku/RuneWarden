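; Damage zone attack that hurts RuneWarden_BP actors either over time or as an area burst.
; By default, sphere overlap starts a looping half-second timer that damages overlapping RuneWardens, cleared when an overlap ends with the zone empty.
; Calling AoEDamage sets IsAoE, which disables the overlap timer logic, then resizes the sphere and applies one hit.
; Both modes send small, knockback-free damage through TakeDamageMessage.
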(event OnComponentBeginOverlap(DamageZone)
  (params (OverlappedComponent :type Primitive%20Component%20Object%20Reference) (OtherActor :type Actor%20Object%20Reference) (OtherComp :type Primitive%20Component%20Object%20Reference) (OtherBodyIndex :type Integer) (bFromSweep :type Boolean) (SweepResult :type Hit%20Result%20Structure%20%28by%20ref%29))
  ;[0.3298 1 0.2087] DoT Damage
  (if (not (Variables|Default|GetisAoE?))
    (bind _returnvalue (Utilities|Time|SetTimerbyEvent (delegate Custom|DoTDamage) 0.5 true))
    (bind _output_get (Variables|Default|SetTimer _returnvalue))))

(event OnComponentEndOverlap(DamageZone)
  (params (OverlappedComponent :type Primitive%20Component%20Object%20Reference) (OtherActor :type Actor%20Object%20Reference) (OtherComp :type Primitive%20Component%20Object%20Reference) (OtherBodyIndex :type Integer))
  ;[0.3298 1 0.2087] DoT Damage
  (if (not (Variables|Default|GetisAoE?))
    (if (Utilities|Array|IsEmpty (Collision|GetOverlappingActors (Variables|Default|GetDamageZone) 0 :!class /Script/Engine.PrimitiveComponent))
      (Utilities|Time|ClearandInvalidateTimerbyHandle (stale OnComponentBeginOverlap(DamageZone) _output_get)))))

(event Custom|DoTDamage
  ;[0.3298 1 0.2087] DoT Damage
  (for _array_element (Collision|GetOverlappingActors (Variables|Default|GetDamageZone) 0 :!class /Script/Engine.PrimitiveComponent)
    (bind _asplayer_character_bp (Utilities|Casting|CastToRuneWarden_BP _array_element))
    (Class|BPIDamagable|TakeDamage(Message) _asplayer_character_bp (Utilities|Struct|MakeBPS_DamageInfo 5.0 0.0 "NewEnumerator4" "NewEnumerator7" "NewEnumerator2") self)))

(event Custom|AoEDamage
  (params (Radius :type Float%20%28double-precision%29))
  (bind _damagezone (Variables|Default|GetDamageZone))
  ;[1 0 0.1223] AoE Damage
  (Variables|Default|SetisAoE? true)
  (if (Variables|Default|GetisAoE?)
    (Components|Sphere|SetSphereRadius _damagezone Radius true)
    (for _array_element (Collision|GetOverlappingActors _damagezone 0 :!class /Script/Engine.PrimitiveComponent)
      (bind _asplayer_character_bp (Utilities|Casting|CastToRuneWarden_BP _array_element))
      (Class|BPIDamagable|TakeDamage(Message) _asplayer_character_bp (Utilities|Struct|MakeBPS_DamageInfo 5.0 0.0 "NewEnumerator4" "NewEnumerator7" "NewEnumerator2") self))))

(event EventBeginPlay
  ;[0.2917 0.2917 0.2917] Event BeginPlay
  (bind _asplayer_character_bp (Utilities|Casting|CastToRuneWarden_BP (Game|Player|GetPlayerPawn 0)))
  (Variables|Default|SetAs%20Player%20Character%20BP _asplayer_character_bp))

(fn ConstructionScript)