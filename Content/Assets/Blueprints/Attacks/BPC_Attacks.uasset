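; Enemy attack component offering melee, projectile, leap, area and damage-over-time attacks, with damage aimed at the RuneWarden player.
; Each attack plays a montage on the owning character and reports start and end through interface messages, most blocking interruption meanwhile.
; Montage notifies trigger melee sphere traces and leap sphere-overlap damage, while projectiles and AoE actors spawn when montages end.
; Leaps launch along a suggested projectile arc; the target-prediction helper is unwired.
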(event Custom|ProjectileAttack
  (params (SpawnTransform :type Transform) (IsHoming :type Boolean) (AttackInfo :type BPS%20Enemy%20Attack%20Info%20Structure))
  (bind (_attacktarget _montagetoplay _damageinfo) (Utilities|Struct|BreakBPS_EnemyAttackInfo AttackInfo))
  (bind _returnvalue (Components|GetOwner))
  ;[0 0.06679 1] Projectile Attack
  (Class|BPIEnemyAI|Attack(Message) _returnvalue _attacktarget)
  (bind _ascharacter (Utilities|Casting|CastToCharacter _returnvalue))
  (Animation|Montage|PlayMontage (Variables|/Script/Engine.Character|GetMesh _ascharacter) _montagetoplay
    (:OnCompleted
      (bind _returnvalue_2 (Game|SpawnActorfromClass "/Game/Assets/Blueprints/Attacks/Projectiles/BP_ProjectileBase.BP_ProjectileBase_C" SpawnTransform "Undefined" "MultiplyWithRoot" _returnvalue 5e+02 0.0 _attacktarget IsHoming 0))
      (EventDispatchers|AssignOnProjectileImpact _returnvalue_2 (delegate Custom|OnProjectileHit))
      (Collision|IgnoreActorwhenMoving (Actor|GetComponentbyClass (Components|GetOwner) "/Script/Engine.CapsuleComponent") _returnvalue_2 true)
      (Class|BPIEnemyAI|AttackEnd(Message) (Components|GetOwner) _attacktarget))
    (:OnInterrupted
      (Class|BPIEnemyAI|AttackEnd(Message) (Components|GetOwner) _attacktarget))))

(event Custom|TestAOEAttack
  (params (BPS_EnemyAttackInfo :type BPS%20Enemy%20Attack%20Info%20Structure%20%28by%20ref%29))
  (bind (_attacktarget _montagetoplay _damageinfo) (Utilities|Struct|BreakBPS_EnemyAttackInfo BPS_EnemyAttackInfo))
  (bind _returnvalue (Components|GetOwner))
  ;[0 1 0.9916] AOE Attack( Currently in Use )
  (Rendering|Debug|DrawDebugSphere (Transformation|GetActorLocation (Components|GetOwner)) 5e+02 12 "(R=1.000000,G=1.000000,B=1.000000,A=1.000000)" 2.0 1.0)
  (bind _outactors (Collision|SphereOverlapActors (Transformation|GetActorLocation _returnvalue) 5e+02 (Utilities|Array|MakeArray "ObjectTypeQuery3") "/Game/Assets/Blueprints/PlayerBP/RuneWarden_BP.RuneWarden_BP_C" (Utilities|Array|MakeArray _returnvalue)))
  (bind _returnvalue_2 (Niagara|SpawnSystemAttached "/Game/Assets/ParticleSystems/Sparks01.Sparks01" (Variables|/Script/Engine.Actor|GetRootComponent (Components|GetOwner)) "None" "0, 0, 0" "0, 0, 0" "KeepRelativeOffset" true))
  (EventDispatchers|AssignOnSystemFinished _returnvalue_2 (delegate Custom|SystemFinished))
  (Audio|PlaySoundatLocation "/Game/Assets/Sounds/Beast/Beast_Damage.Beast_Damage" (Transformation|GetActorLocation (Components|GetOwner)) "0, 0, 0" 1.0 1.0 0.0 0 0 0 0)
  (for _array_element _outactors
    (Class|BPIDamagable|TakeDamage(Message) _array_element _damageinfo (Components|GetOwner))
    (Class|BPIEnemyAI|AttackEnd(Message) _array_element _attacktarget)))

(event Custom|OnLand
  (params (Hit :type Hit%20Result%20Structure%20%28by%20ref%29))
  ;[0 1 0.008637] Jump To Target Actor location with arc with / without prediction
  (EventDispatchers|UnbindEventfromLandedDelegate (stale Custom|JumpToAttackTarget _ascharacter) (delegate Custom|OnLand))
  (Components|Movement|StopMovementImmediately (Actor|GetComponentbyClass (Components|GetOwner) "/Script/Engine.CharacterMovementComponent")))

(event Custom|AttackTemplpate
  (params (AttackInfo :type BPS%20Enemy%20Attack%20Info%20Structure))
  (bind (_attacktarget _montagetoplay) (Utilities|Struct|BreakBPS_EnemyAttackInfo AttackInfo))
  (bind _returnvalue (Components|GetOwner))
  (bind _returnvalue_2 (Components|GetOwner))
  ;[1 0.8181 0] Attack Template
  (Class|BPIEnemyAI|Attack(Message) _returnvalue _attacktarget)
  (bind _ascharacter (Utilities|Casting|CastToCharacter _returnvalue))
  (Animation|Montage|PlayMontage (Variables|/Script/Engine.Character|GetMesh _ascharacter) _montagetoplay
    (:then
      (Class|BPIDamagable|SetIsInterruptible(Message) _returnvalue_2 false))
    (:OnCompleted
      (Class|BPIEnemyAI|AttackEnd(Message) _returnvalue_2 _attacktarget :!label _label)
      (Class|BPIDamagable|SetIsInterruptible(Message) _returnvalue_2 true))
    (:OnInterrupted
      (goto _label))))

(event Custom|DoTAttack
  (params (AttackInfo :type BPS%20Enemy%20Attack%20Info%20Structure))
  (bind (_attacktarget _montagetoplay) (Utilities|Struct|BreakBPS_EnemyAttackInfo AttackInfo))
  (bind _returnvalue (Components|GetOwner))
  (bind _returnvalue_2 (Components|GetOwner))
  ;[1 0.3345 0.89] DoT Attack
  (Class|BPIEnemyAI|Attack(Message) _returnvalue _attacktarget)
  (bind _ascharacter (Utilities|Casting|CastToCharacter _returnvalue))
  (Animation|Montage|PlayMontage (Variables|/Script/Engine.Character|GetMesh _ascharacter) _montagetoplay
    (:then
      (Class|BPIDamagable|SetIsInterruptible(Message) _returnvalue_2 false))
    (:OnCompleted
      (Game|SpawnActorfromClass "/Game/Assets/Blueprints/Attacks/BP_DoT_AoE.BP_DoT_AoE_C" (Transformation|GetActorTransform _returnvalue_2) "Undefined" "MultiplyWithRoot" 0 0 :!label _label)
      (Class|BPIEnemyAI|AttackEnd(Message) _returnvalue_2 _attacktarget)
      (Class|BPIDamagable|SetIsInterruptible(Message) _returnvalue_2 true))
    (:OnInterrupted
      (goto _label))))

(event Custom|MeleeAttack
  (params (TraceStart :type Vector) (TraceEnd :type Vector) (AttackInfo :type BPS%20Enemy%20Attack%20Info%20Structure) (Radius :type Float%20%28single-precision%29))
  (bind (_attacktarget _montagetoplay _damageinfo) (Utilities|Struct|BreakBPS_EnemyAttackInfo AttackInfo))
  (bind _returnvalue (Components|GetOwner))
  ;[1 0 0] Melee Attack
  (Class|BPIEnemyAI|Attack(Message) _returnvalue _attacktarget)
  (bind _ascharacter (Utilities|Casting|CastToCharacter _returnvalue))
  (bind _notifyname (Animation|Montage|PlayMontage (Variables|/Script/Engine.Character|GetMesh _ascharacter) _montagetoplay)
    (:then
      (Class|BPIDamagable|SetIsInterruptible(Message) _returnvalue false))
    (:OnCompleted
      (Class|BPIEnemyAI|AttackEnd(Message) _returnvalue _attacktarget :!label _label)
      (Class|BPIDamagable|SetIsInterruptible(Message) _returnvalue true))
    (:OnInterrupted
      (goto _label))
    (:OnNotifyBegin
      (switch name _notifyname
        (:Attack_trace
          (CallFunction|SphereTraceDamage TraceStart TraceEnd _damageinfo Radius _attacktarget))))))

(event Custom|AoeAttack
  (params (AttackInfo :type BPS%20Enemy%20Attack%20Info%20Structure))
  (bind (_attacktarget _montagetoplay) (Utilities|Struct|BreakBPS_EnemyAttackInfo AttackInfo))
  (bind _returnvalue (Components|GetOwner))
  (bind _returnvalue_2 (Components|GetOwner))
  ;[1 1 1] AoE Attack
  (Class|BPIEnemyAI|Attack(Message) _returnvalue_2 _attacktarget)
  (bind _ascharacter (Utilities|Casting|CastToCharacter _returnvalue_2))
  (Animation|Montage|PlayMontage (Variables|/Script/Engine.Character|GetMesh _ascharacter) _montagetoplay
    (:then
      (Class|BPIDamagable|SetIsInterruptible(Message) _returnvalue false))
    (:OnCompleted
      (bind _returnvalue_3 (Game|SpawnActorfromClass "/Game/Assets/Blueprints/Attacks/BP_DoT_AoE.BP_DoT_AoE_C" (Transformation|GetActorTransform _returnvalue) "Undefined" "MultiplyWithRoot" 0 0 :!label _label))
      (Default|AoEDamage _returnvalue_3 6e+02)
      (Class|BPIEnemyAI|AttackEnd(Message) _returnvalue _attacktarget)
      (Class|BPIDamagable|SetIsInterruptible(Message) _returnvalue true))
    (:OnInterrupted
      (goto _label))))

(event Custom|LeapAttack
  (params (AttackInfo :type BPS%20Enemy%20Attack%20Info%20Structure) (ArcHeight :type Float%20%28double-precision%29))
  (bind (_attacktarget _montagetoplay _damageinfo) (Utilities|Struct|BreakBPS_EnemyAttackInfo AttackInfo))
  (bind _returnvalue (Components|GetOwner))
  ;[1 0 0] Leap Attack (Change Melee attack to jump attack animation)
  (Class|BPIEnemyAI|Attack(Message) _returnvalue _attacktarget)
  (CallFunction|JumptoAttackTarget _attacktarget ArcHeight)
  (bind _ascharacter (Utilities|Casting|CastToCharacter _returnvalue))
  (bind _notifyname (Animation|Montage|PlayMontage (Variables|/Script/Engine.Character|GetMesh _ascharacter) _montagetoplay)
    (:then
      (Class|BPIDamagable|SetIsInterruptible(Message) _returnvalue false))
    (:OnCompleted
      (Class|BPIEnemyAI|AttackEnd(Message) (Components|GetOwner) _attacktarget :!label _label)
      (Class|BPIDamagable|SetIsInterruptible(Message) _returnvalue true))
    (:OnInterrupted
      (goto _label))
    (:OnNotifyBegin
      (switch name _notifyname
        (:Attack_trace
          (CallFunction|TestAOEAttack (Utilities|Struct|MakeBPS_EnemyAttackInfo _attacktarget _montagetoplay _damageinfo)))))))

(event Custom|OnProjectileHit
  (params (OtherActor :type Actor%20Object%20Reference) (Hit :type Hit%20Result%20Structure))
  (bind _returnvalue (Components|GetOwner))
  ;[0 0.06679 1] Projectile Attack
  (bind _asrune_warden_bp (Utilities|Casting|CastToRuneWarden_BP OtherActor))
  (Class|BPIDamagable|TakeDamage(Message) _asrune_warden_bp (.DamageInfo (Utilities|Struct|BreakBPS_EnemyAttackInfo (stale Custom|ProjectileAttack AttackInfo))) _returnvalue)
  (Class|AISenseDamage|ReportDamageEvent _asrune_warden_bp _returnvalue (.Amount (Utilities|Struct|BreakBPS_DamageInfo (.DamageInfo (Utilities|Struct|BreakBPS_EnemyAttackInfo (stale Custom|ProjectileAttack AttackInfo))))) (Transformation|GetActorLocation (Components|GetOwner)) "0, 0, 0" "None"))

(event Custom|SphereTraceDamage
  (params (Start :type Vector) (End :type Vector) (DamageInfo :type BPS%20Damage%20Info%20Structure) (Radius :type Float%20%28single-precision%29) (AttackTarget :type Actor%20Object%20Reference))
  (bind _returnvalue (Components|GetOwner))
  ;[0.2844 0.2844 0.2844] Attack Notifies
  ;;[0.9969 0.6313 0] Sphere Trace
  (bind _outactors (Actor|GetAllActorsOfClass "/Game/Assets/Blueprints/EnemyBP/GeneralEnemyBPs/EnemyBP.EnemyBP_C"))
  (bind (_outhit _returnvalue_2) (Collision|SphereTraceForObjects Start End Radius (Utilities|Array|MakeArray "ObjectTypeQuery3") false _outactors "ForDuration" true "(R=0.000000,G=0.958806,B=1.000000,A=1.000000)" "(R=0.963357,G=1.000000,B=0.000000,A=1.000000)" 1.0))
  (if _returnvalue_2
    (Class|BPIDamagable|TakeDamage(Message) (.HitActor (Collision|BreakHitResult _outhit)) DamageInfo _returnvalue)
    (Class|BPIEnemyAI|AttackEnd(Message) _returnvalue AttackTarget)))

(event Custom|JumpToAttackTarget
  (params (AttackTarget :type Actor%20Object%20Reference) (ArcHeight :type Float%20%28double-precision%29))
  (bind _returnvalue (Transformation|GetActorLocation AttackTarget))
  ;[0 1 0.008637] Jump To Target Actor location with arc with / without prediction
  (bind _outlaunchvelocity (Game|SuggestProjectileVelocityCustomArc (Transformation|GetActorLocation (Components|GetOwner)) (Math|Vector|MakeVector (.x _returnvalue) (.y _returnvalue) (+ (.z _returnvalue) -5e+01)) 0.0 ArcHeight))
  (bind _ascharacter (Utilities|Casting|CastToCharacter (Components|GetOwner)))
  (Character|LaunchCharacter _ascharacter _outlaunchvelocity true true)
  (EventDispatchers|BindEventtoLandedDelegate _ascharacter (delegate Custom|OnLand)))

(event Custom|SystemFinished
  (params (PSystem :type Niagara%20Component%20Object%20Reference))
  ;[0 1 0.9916] AOE Attack( Currently in Use )
  (Components|DestroyComponent PSystem))

(fn CalculateFutureActorLocation
  (params (Actor :type Actor%20Object%20Reference) (Time :type Float%20%28double-precision%29))
  ;[1 1 1] TargetLocation = Velocity * Time + CurrentLocation
  (return (+ (Transformation|GetActorLocation Actor) (* (* (Transformation|GetVelocity Actor) "1.000000,1.000000,0.000000") Time))))