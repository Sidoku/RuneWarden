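; Player combat component for the RuneWarden character, handling light, aerial and heavy combos, block, roll dodge and aura overlays.
; Attacks play montages from indexed combo arrays, with notifies reopening the attack window, completion or delayed interruption resetting indices, and damage data setting staff socket and aura.
; A preceding light attack shifts the heavy combo's starting index.
; Skill selection swaps light combos, but heavy attacks always use the kick set.
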(event Custom|AirLightAttack
  (bind _playerref (Variables|Default|GetPlayerRef))
  (bind _playerref_2 (Variables|Default|GetPlayerRef))
  (bind _charactermovement (Variables|/Script/Engine.Character|GetCharacterMovement _playerref))
  ;[0 0.09053 1] Air Light Attack Combo(Fix disabling constraint disabling does not work properly)
  (Class|MovementComponent|SetPlaneConstraintAxisSetting _charactermovement "Z")
  (Class|MovementComponent|SetPlaneConstraintEnabled _charactermovement true)
  (Variables|/Game/Assets/Blueprints/PlayerBP/RuneWarden_BP.RuneWarden_BP_C|SetCurrentPlayerState (Variables|Default|GetPlayerRef) "NewEnumerator2")
  (bind _output_get (Variables|Default|SetDamageInfo (.bpsdamageinfo (Utilities|Array|Get(acopy) (Variables|Default|GetAirLightAttackCombo) (Variables|Default|GetLightAttackIndex)))))
  (CallFunction|EquipStaff (.staffequipped? _output_get))
  (Animation|Montage|PlayMontage (Variables|/Script/Engine.Character|GetMesh _playerref) (.attackmontage (Utilities|Array|Get(acopy) (Variables|Default|GetAirLightAttackCombo) (Variables|Default|GetLightAttackIndex)))
    (:then
      (bind _result (Math|Integer|IncrementInt (Variables|Default|GetLightAttackIndex))
        (:%20%20
          (Variables|Default|SetLightAttackIndex _result)
          (Variables|Default|SetwasLightAttack? true))))
    (:OnCompleted
      (Class|MovementComponent|SetPlaneConstraintEnabled _charactermovement false :!pinned true) ; Fix
      (Variables|Default|SetLightAttackIndex 0)
      (Variables|Default|SetwasLightAttack? false)
      (Variables|/Game/Assets/Blueprints/PlayerBP/RuneWarden_BP.RuneWarden_BP_C|SetCanAttack _playerref_2 true :!label _label)
      (Variables|/Game/Assets/Blueprints/PlayerBP/RuneWarden_BP.RuneWarden_BP_C|SetAttacking _playerref_2 false)
      (Variables|/Game/Assets/Blueprints/PlayerBP/RuneWarden_BP.RuneWarden_BP_C|SetCurrentPlayerState (Variables|Default|GetPlayerRef) "NewEnumerator4"))
    (:OnInterrupted
      (Utilities|FlowControl|RetriggerableDelay 3.0)
      (Variables|Default|SetLightAttackIndex 0)
      (goto _label))
    (:OnNotifyBegin
      (goto _label))))

(event Custom|OnHeavyAttack
  (bind _playerref (Variables|Default|GetPlayerRef))
  (bind _playerref_2 (Variables|Default|GetPlayerRef))
  (bind _charactermovement (Variables|/Script/Engine.Character|GetCharacterMovement _playerref_2))
  ;[1 0 0.1033] Heavy Attack Combo
  (Default|AddImpulse _playerref_2)
  (Variables|/Script/Engine.CharacterMovementComponent|SetMaxWalkSpeed _charactermovement 4e+02)
  (Variables|/Game/Assets/Blueprints/PlayerBP/RuneWarden_BP.RuneWarden_BP_C|SetCurrentPlayerState (Variables|Default|GetPlayerRef) "NewEnumerator2")
  (if (Variables|Default|GetwasLightAttack?)
    (Variables|Default|SetHeavyAttackIndex 1))
  (bind _output_get (Variables|Default|SetDamageInfo (.bpsdamageinfo (Utilities|Array|Get(acopy) (Variables|Default|GetKickAttackHeavy) (Variables|Default|GetHeavyAttackIndex)))))
  (CallFunction|EquipStaff (.staffequipped? _output_get))
  (Animation|Montage|PlayMontage (Variables|/Script/Engine.Character|GetMesh _playerref_2) (.attackmontage (Utilities|Array|Get(acopy) (Variables|Default|GetKickAttackHeavy) (Variables|Default|GetHeavyAttackIndex)))
    (:then
      (bind _result (Math|Integer|IncrementInt (Variables|Default|GetHeavyAttackIndex))
        (:%20%20
          (Variables|Default|SetHeavyAttackIndex _result)
          (Variables|Default|SetwasLightAttack? false))))
    (:OnCompleted
      (Variables|/Script/Engine.CharacterMovementComponent|SetMaxWalkSpeed _charactermovement 8e+02)
      (Variables|Default|SetHeavyAttackIndex 0 :!label _label)
      (Variables|/Game/Assets/Blueprints/PlayerBP/RuneWarden_BP.RuneWarden_BP_C|SetCanAttack _playerref true :!label _label_2)
      (Variables|/Game/Assets/Blueprints/PlayerBP/RuneWarden_BP.RuneWarden_BP_C|SetAttacking _playerref false)
      (Variables|/Game/Assets/Blueprints/PlayerBP/RuneWarden_BP.RuneWarden_BP_C|SetCurrentPlayerState (Variables|Default|GetPlayerRef) "NewEnumerator4"))
    (:OnInterrupted
      (Utilities|FlowControl|RetriggerableDelay 3.0)
      (goto _label))
    (:OnNotifyBegin
      (goto _label_2))))

(event Custom|OnLightAttack
  (bind _playerref (Variables|Default|GetPlayerRef))
  (bind _playerref_2 (Variables|Default|GetPlayerRef))
  ;[0.04616 1 0.03639] Light Attack Combo
  (Default|AddImpulse _playerref)
  (Variables|/Game/Assets/Blueprints/PlayerBP/RuneWarden_BP.RuneWarden_BP_C|SetCurrentPlayerState (Variables|Default|GetPlayerRef) "NewEnumerator2")
  (bind _output_get (Variables|Default|SetDamageInfo (.bpsdamageinfo (Utilities|Array|Get(acopy) (Variables|Default|GetLightAttackCombo) (Variables|Default|GetLightAttackIndex)))))
  (CallFunction|EquipStaff (.staffequipped? _output_get))
  (Animation|Montage|PlayMontage (Variables|/Script/Engine.Character|GetMesh _playerref) (.attackmontage (Utilities|Array|Get(acopy) (Variables|Default|GetLightAttackCombo) (Variables|Default|GetLightAttackIndex)))
    (:then
      (bind _result (Math|Integer|IncrementInt (Variables|Default|GetLightAttackIndex))
        (:%20%20
          (Variables|Default|SetLightAttackIndex _result)
          (Variables|Default|SetwasLightAttack? true))))
    (:OnCompleted
      (Variables|/Script/Engine.CharacterMovementComponent|SetMaxWalkSpeed (Variables|/Script/Engine.Character|GetCharacterMovement _playerref) 8e+02)
      (Variables|Default|SetLightAttackIndex 0)
      (Variables|Default|SetwasLightAttack? false)
      (Variables|/Game/Assets/Blueprints/PlayerBP/RuneWarden_BP.RuneWarden_BP_C|SetCanAttack _playerref_2 true :!label _label)
      (Variables|/Game/Assets/Blueprints/PlayerBP/RuneWarden_BP.RuneWarden_BP_C|SetAttacking _playerref_2 false)
      (Variables|/Game/Assets/Blueprints/PlayerBP/RuneWarden_BP.RuneWarden_BP_C|SetCurrentPlayerState (Variables|Default|GetPlayerRef) "NewEnumerator4"))
    (:OnInterrupted
      (Utilities|FlowControl|RetriggerableDelay 3.0)
      (Variables|Default|SetLightAttackIndex 0)
      (goto _label))
    (:OnNotifyBegin
      (goto _label))))

(event Custom|AuraOverlay
  (bind _playerref (Variables|Default|GetPlayerRef))
  (bind _mesh (Variables|/Script/Engine.Character|GetMesh _playerref))
  ;[0.6487 0.6273 1] Aura Overlay
  (switch Utilities|FlowControl|Switch|SwitchonBPE_AuraType (.AuraType (Utilities|Struct|BreakBPS_DamageInfo (Variables|Default|GetDamageInfo)))
    (:NewEnumerator0
      (Rendering|Material|SetOverlayMaterial _mesh "/Game/Assets/Materials/MaterialInstances/MI_Player/MI_CalmAura.MI_CalmAura" :!class /Script/Engine.MeshComponent))
    (:NewEnumerator1
      (Rendering|Material|SetOverlayMaterial _mesh "/Game/Assets/Materials/MaterialInstances/MI_Player/MI_RageAura.MI_RageAura" :!class /Script/Engine.MeshComponent))
    (:NewEnumerator2
      (Rendering|Material|SetOverlayMaterial _mesh "/Game/Assets/Materials/MaterialInstances/MI_Player/MI_GreenAura.MI_GreenAura" :!class /Script/Engine.MeshComponent))
    (:NewEnumerator3
      (Rendering|Material|SetOverlayMaterial _mesh "/Game/Assets/Materials/MaterialInstances/MI_Player/MI_YellowAura.MI_YellowAura" :!class /Script/Engine.MeshComponent))))

(event Custom|SwitchAttack
  ;[1 1 1] Test combo switching
  (Utilities|FlowControl|FlipFlop
    (:A
      (Variables|Default|SetLightAttackCombo (Variables|Default|GetStaffAttackLight))
      (Development|PrintString "Kick Attack"))
    (:B
      (Variables|Default|SetLightAttackCombo (Variables|Default|GetPunchAttackLight))
      (Development|PrintString "Punch Attack"))))

(event Custom|Dodge
  (bind _playerref (Variables|Default|GetPlayerRef))
  (bind _playerref_2 (Variables|Default|GetPlayerRef))
  ;[0.277 0.3519 1] Dodge / Roll Need to fix invincibility
  (Development|PrintString "dodging")
  (Default|SetIsInvincible _playerref_2 true)
  (Variables|/Script/Engine.CharacterMovementComponent|SetMaxWalkSpeed (Variables|/Script/Engine.Character|GetCharacterMovement _playerref_2) 6e+02)
  (Variables|/Game/Assets/Blueprints/PlayerBP/RuneWarden_BP.RuneWarden_BP_C|SetCurrentPlayerState _playerref_2 "NewEnumerator3")
  (Animation|Montage|PlayMontage (Variables|/Script/Engine.Character|GetMesh _playerref_2) "/Game/Assets/Player/Animations/A_Montages/Final_Montages/RuneWarden_Roll_Montage.RuneWarden_Roll_Montage"
    (:OnCompleted
      (Variables|/Game/Assets/Blueprints/PlayerBP/RuneWarden_BP.RuneWarden_BP_C|SetCurrentPlayerState _playerref "NewEnumerator1")
      (Variables|/Script/Engine.CharacterMovementComponent|SetMaxWalkSpeed (Variables|/Script/Engine.Character|GetCharacterMovement _playerref) 8e+02)
      (Default|SetIsInvincible _playerref false)
      (Utilities|FlowControl|Delay 0.7)
      (Variables|/Game/Assets/Blueprints/PlayerBP/RuneWarden_BP.RuneWarden_BP_C|SetCanAttack _playerref true)
      (Variables|/Game/Assets/Blueprints/PlayerBP/RuneWarden_BP.RuneWarden_BP_C|SetCanDodge _playerref true))))

(event Custom|SelectSkill
  (params (CurrentSkill :type String))
  ;[1 0.8704 0] Select the skill based on user selection from UI
  (switch string CurrentSkill
    (:KickAttackLight
      (Variables|Default|SetLightAttackCombo (Variables|Default|GetStaffAttackLight))
      (Development|PrintString "Staff Attack"))
    (:PunchAttackLight
      (Variables|Default|SetLightAttackCombo (Variables|Default|GetPunchAttackLight))
      (Development|PrintString "Light Attack"))
    (:PunchHeavy
      (Variables|Default|SetHeavyAttackCombo (Variables|Default|GetPunchHeavy)))))

(event Custom|StaffDelay
  ;[1 0.2917 0.2917] Timed Upequip Staff
)

(event Custom|EquipStaff
  (params (Staff? :type Boolean))
  (bind _playerref (Variables|Default|GetPlayerRef))
  (bind _staff (Variables|/Game/Assets/Blueprints/PlayerBP/RuneWarden_BP.RuneWarden_BP_C|GetStaff _playerref))
  (bind _mesh (Variables|/Script/Engine.Character|GetMesh _playerref))
  ;[0.3021 1 1] Equip Staff
  (if Staff?
    (Transformation|AttachComponentToComponent _staff _mesh "EquipStaff" "SnapToTarget" "SnapToTarget" "SnapToTarget" true)
    (else
      (Transformation|AttachComponentToComponent _staff _mesh "UnequipStaff" "SnapToTarget" "SnapToTarget" "SnapToTarget" true))))

(event Custom|StartBlock
  (bind _playerref (Variables|Default|GetPlayerRef))
  ;[1 1 1] Block
  (Utilities|FlowControl|DoOnce false
    (:Completed
      (Animation|Montage|PlayMontage (Variables|/Script/Engine.Character|GetMesh _playerref) "/Game/Assets/Player/Animations/A_Montages/Final_Montages/RuneWarden_Hit_Montage.RuneWarden_Hit_Montage"
        (:OnCompleted
          (CallFunction|EndBlock))
        (:OnInterrupted
          (if (not (Variables|/Game/Assets/Blueprints/PlayerBP/RuneWarden_BP.RuneWarden_BP_C|GetIsReactingToBlock _playerref))
            (CallFunction|EndBlock)))
        (:OnNotifyBegin
          (Variables|/Game/Assets/DamageSystem/BPC_DamageSystem.BPC_DamageSystem_C|SetIsBlocking (Variables|/Game/Assets/Blueprints/PlayerBP/RuneWarden_BP.RuneWarden_BP_C|GetBPC_DamageSystem (Variables|Default|GetPlayerRef)) true))))))

(event Custom|Reset%20Block
  (bind _playerref (Variables|Default|GetPlayerRef))
  ;[1 1 1] Block
  (Utilities|FlowControl|DoOnce false) ; enters at Reset
)

(event Custom|EndBlock
  (bind _playerref (Variables|Default|GetPlayerRef))
  ;[1 1 1] Block
  (Variables|/Game/Assets/DamageSystem/BPC_DamageSystem.BPC_DamageSystem_C|SetIsBlocking (Variables|/Game/Assets/Blueprints/PlayerBP/RuneWarden_BP.RuneWarden_BP_C|GetBPC_DamageSystem _playerref) false)
  (Variables|/Game/Assets/Blueprints/PlayerBP/RuneWarden_BP.RuneWarden_BP_C|SetCanAttack _playerref true)
  (Variables|/Game/Assets/Blueprints/PlayerBP/RuneWarden_BP.RuneWarden_BP_C|SetCanDodge _playerref false)
  (Variables|/Game/Assets/Blueprints/PlayerBP/RuneWarden_BP.RuneWarden_BP_C|SetIsReactingToBlock _playerref false)
  (CallFunction|ResetBlock)
  (Animation|StopAnimMontage _playerref 0))

(event EventBeginPlay
  ;[1 1 1] Set Player Reference
  (bind _asrune_warden_bp (Utilities|Casting|CastToRuneWarden_BP (Game|Player|GetPlayerPawn 0)))
  (Variables|Default|SetPlayerRef _asrune_warden_bp)
  ;[1 1 1] Initialize first combo
  (Variables|Default|SetLightAttackCombo (Variables|Default|GetStaffAttackLight)) ; Staff
  (Development|PrintString "Kick Attack")
  ;[1 1 1] Equip Staff
  (CallFunction|EquipStaff false))