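; BP_SaveState toggles the player's skill inventory screen; despite its name, its graph contains no save logic.
; BeginPlay caches the PlayerCharacterBP pawn and creates a WB_Inventory widget once.
; The SkillInventory event uses a FlipFlop to show the widget, disable character movement and enable cursor with game-and-UI input, or to remove it and restore walking and game-only input.
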(event Custom|Begin%20Play
  (bind _asplayer_character_bp (Utilities|Casting|CastToPlayerCharacterBP (Game|Player|GetPlayerPawn 0)))
  (Variables|Default|SetPlayerRef _asplayer_character_bp)
  (bind _returnvalue (UserInterface|CreateWidget "/Game/Inventory/WB_Inventory.WB_Inventory_C" (Game|GetPlayerController 0)))
  (Variables|Default|SetSkillInventory _returnvalue))

(event Custom|Skill%20Inventory
  (bind _returnvalue (Game|GetPlayerController 0))
  (bind _returnvalue_2 (Game|GetPlayerController 0))
  (Utilities|FlowControl|FlipFlop
    (:A
      (UserInterface|Viewport|AddtoViewport (Variables|Default|GetSkillInventory) 0)
      (Pawn|Components|CharacterMovement|SetMovementMode (Variables|/Script/Engine.Character|GetCharacterMovement (Variables|Default|GetPlayerRef)) "MOVE_None" 0)
      (Input|SetInputModeGameandUI _returnvalue (Variables|Default|GetSkillInventory) "DoNotLock" true false)
      (Variables|/Script/Engine.PlayerController|SetbShowMouseCursor _returnvalue true))
    (:B
      (Widget|RemovefromParent (Variables|Default|GetSkillInventory))
      (Pawn|Components|CharacterMovement|SetMovementMode (Variables|/Script/Engine.Character|GetCharacterMovement (Variables|Default|GetPlayerRef)) "MOVE_Walking" 0)
      (Input|SetInputModeGameOnly _returnvalue_2 false)
      (Variables|/Script/Engine.PlayerController|SetbShowMouseCursor _returnvalue_2 false))))