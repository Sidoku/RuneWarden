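; Toothy enemy Blueprint that defines the creature's melee and leap attacks against a given target.
; Both attack events pack the target, a Toothy montage and damage info into an attack struct and pass it to the BPCAttacks component.
; Melee supplies a short trace ahead of the actor, while the harder-hitting leap supplies an arc height, and neither applies knockback.
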(event Custom|MeleeAttack
  (params (AttackTarget :type Actor%20Object%20Reference))
  (bind _returnvalue (Transformation|GetActorLocation))
  ;[1 1 1] Melee Attack
  (Default|MeleeAttack (Variables|Default|GetBPC_Attacks) _returnvalue (+ _returnvalue (* (Transformation|GetActorForwardVector) 1e+02)) (Utilities|Struct|MakeBPS_EnemyAttackInfo AttackTarget "/Game/Assets/Enemies/Toothy/Toothy1_Attack_Montage.Toothy1_Attack_Montage" (Utilities|Struct|MakeBPS_DamageInfo 2e+01 0.0 "NewEnumerator1")) 5e+01))

(event Custom|LeapAttack
  (params (AttackTarget :type Actor%20Object%20Reference))
  ;[1 1 1] Leap Attack
  (Default|LeapAttack (Variables|Default|GetBPC_Attacks) (Utilities|Struct|MakeBPS_EnemyAttackInfo AttackTarget "/Game/Assets/Enemies/Toothy/Toothy1_Attack2_Montage.Toothy1_Attack2_Montage" (Utilities|Struct|MakeBPS_DamageInfo 3e+01 0.0 "NewEnumerator1")) 0.7))

(event EventBeginPlay
  (|CallParentFunction) ; This node is disabled and will not be called.\nDrag off pins to build functionality.
)

(event Collision|EventActorBeginOverlap
  (params (OtherActor :type Actor%20Object%20Reference)))

(event EventTick
  (params (DeltaSeconds :type Float%20%28single-precision%29)))

(fn ConstructionScript
  (|CallParentFunction))