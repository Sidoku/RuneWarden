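; Trigger-box enemy spawner that starts a one-time combat encounter when overlapped.
; Overlap briefly freezes the player, spawns a BP_CombatZone, then after PortalTimer spawns one to four enemies in a row ahead of the player.
; Enemies cycle through four class slots via MultiGate, are projected onto the navmesh facing the player, and receive a spawner reference.
; DeathSpawnCount tallies deaths and destroys the zone and spawner when all are dead.
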(event OnComponentBeginOverlap(Box)
  (params (OverlappedComponent :type Primitive%20Component%20Object%20Reference) (OtherActor :type Actor%20Object%20Reference) (OtherComp :type Primitive%20Component%20Object%20Reference) (OtherBodyIndex :type Integer) (bFromSweep :type Boolean) (SweepResult :type Hit%20Result%20Structure%20%28by%20ref%29))
  (bind _returnvalue (Game|GetPlayerCharacter 0))
  (bind _returnvalue_2 (Game|GetPlayerCharacter 0))
  (bind _spawn_count (Variables|Default|GetSpawn%20Count))
  (bind _spawn_count_2 (Variables|Default|GetSpawn%20Count))
  (bind _portaltimer (Variables|Default|GetPortalTimer))
  (bind _returnvalue_3 (Transformation|GetActorLocation _returnvalue))
  (bind _returnvalue_4 (- _spawn_count_2 1))
  (bind _charactermovement (Variables|/Script/Engine.Character|GetCharacterMovement _returnvalue_2))
  ;[1 0.04388 0.1636] Spawner Code
  (Utilities|FlowControl|DoOnce false
    (:Completed
      (Utilities|FlowControl|Sequence
        (:then_0
          ;[1 0.1087 0.7842] Combat Zone
          (Pawn|Components|CharacterMovement|SetMovementMode _charactermovement "MOVE_None" 0)
          (Utilities|FlowControl|Delay 0.5)
          (bind _returnvalue_5 (Game|SpawnActorfromClass "/Game/Levels/BlockMesh_Assets/BP_CombatZone.BP_CombatZone_C" (Math|Transform|MakeTransform (Transformation|GetWorldLocation (Variables|Default|GetPortal%20Spawn%20Point)) "0, 0, 0" (Variables|Default|GetCombatZoneSize)) "Undefined" "MultiplyWithRoot" 0 0))
          (Pawn|Components|CharacterMovement|SetMovementMode _charactermovement "MOVE_Walking" 0))
        (:then_1
          (Utilities|FlowControl|Delay _portaltimer)
          (if (== _spawn_count 1)
            (Variables|Default|SetOffset%20Spawn%20Enemy 0.0)
            (for _index (range 0 _returnvalue_4) :!label _label
              (Utilities|FlowControl|MultiGate false true 0
                (:Out%200
                  (Variables|Default|SetEnemyRef (Variables|Default|GetEnemy%20Ref_1)))
                (:Out%201
                  (Variables|Default|SetEnemyRef (Variables|Default|GetEnemy%20Ref_2)))
                (:Out%202
                  (Variables|Default|SetEnemyRef (Variables|Default|GetEnemy%20Ref_3)))
                (:Out%203
                  (Variables|Default|SetEnemyRef (Variables|Default|GetEnemy%20Ref_4))))
              (bind _returnvalue_6 (Game|SpawnActorfromClass (Variables|Default|GetEnemyRef) (Math|Transform|MakeTransform (.ProjectedLocation (AI|Navigation|ProjectPointtoNavigation (+ _returnvalue_3 (* (Transformation|GetActorForwardVector _returnvalue) (Variables|Default|GetPlayer%20to%20Enemy)) (* (Transformation|GetActorRightVector _returnvalue) (* (+ (- _index _returnvalue_4) (Variables|Default|GetOffset%20Spawn%20Enemy)) (Variables|Default|GetEnemySeperation)))) 0 0 "0, 0, 0")) (Math|Rotator|FindLookatRotation (.ProjectedLocation (AI|Navigation|ProjectPointtoNavigation (+ _returnvalue_3 (* (Transformation|GetActorForwardVector _returnvalue) (Variables|Default|GetPlayer%20to%20Enemy)) (* (Transformation|GetActorRightVector _returnvalue) (* (+ (- _index _returnvalue_4) (Variables|Default|GetOffset%20Spawn%20Enemy)) (Variables|Default|GetEnemySeperation)))) 0 0 "0, 0, 0")) _returnvalue_3) "1.000000,1.000000,1.000000") "AdjustIfPossibleButAlwaysSpawn" "MultiplyWithRoot" 0 0))
              (bind _asenemy_bp (Utilities|Casting|CastToEnemyBP _returnvalue_6))
              (Variables|/Game/Assets/Blueprints/EnemyBP/GeneralEnemyBPs/EnemyBP.EnemyBP_C|SetBPSpawnerRef _asenemy_bp self))))
        (:then_2
          (Utilities|FlowControl|Delay _portaltimer)
          (if (== _spawn_count 2)
            (Variables|Default|SetOffset%20Spawn%20Enemy 0.5)
            (goto _label)))
        (:then_3
          (Utilities|FlowControl|Delay _portaltimer)
          (if (== _spawn_count 3)
            (Variables|Default|SetOffset%20Spawn%20Enemy 1.0)
            (goto _label)))
        (:then_4
          (Utilities|FlowControl|Delay _portaltimer)
          (if (== _spawn_count 4)
            (Variables|Default|SetOffset%20Spawn%20Enemy 1.5)
            (goto _label)))))))

(event EventDeathSpawnCount
  (bind _deathcounter (Variables|Default|GetDeathCounter))
  (bind _result (Math|Integer|IncrementInt _deathcounter)
    (:%20%20
      (if (== _result (Variables|Default|GetSpawn%20Count))
        ;[1 1 1] Frankie spawner collision zone section
        (Development|PrintString "All spawned enemies are dead")
        ;[1 1 1] Destory spawner and combat sphere
        (Actor|DestroyActor (stale OnComponentBeginOverlap(Box) _returnvalue_5))
        (Actor|DestroyActor)
        (else
          (Development|PrintString (Utilities|String|ToString(Integer) _deathcounter)))))))

(event EventBeginPlay
  (bind _asbp_game_instance (Utilities|Casting|CastToBP_GameInstance (Game|GetGameInstance)))
  (Variables|Default|SetAs%20BP%20Game%20Instance _asbp_game_instance)
  (bind _asrune_warden_bp (Utilities|Casting|CastToRuneWardenBP (Game|GetGameMode)))
  (Variables|Default|SetAs%20Rune%20Warden%20BP _asrune_warden_bp)
  (bind _returnvalue (Actor|GetActorOfClass (Variables|Default|GetEnemyRef)))
  (bind _asenemy_bp (Utilities|Casting|CastToEnemyBP _returnvalue))
  (Variables|/Game/Assets/Blueprints/EnemyBP/GeneralEnemyBPs/EnemyBP.EnemyBP_C|SetPortalSize _asenemy_bp (Variables|Default|GetPortalSize)))

(fn ConstructionScript)

(fn Block
  (params (CanBlock? :type Boolean) (BlockDamage :type Float%20%28double-precision%29) (BlockBroken? :type Boolean))
  (return false false))

(fn KnockBack
  (params (CanKnockBack? :type Boolean) (KnockBackDistance :type Float%20%28double-precision%29))
  (return false))

(fn Stagger
  (params (CanStagger? :type Boolean))
  (return false))

(fn Target
  (params (CanTarget? :type Boolean) (TargetDistance :type Float%20%28double-precision%29))
  (return false))