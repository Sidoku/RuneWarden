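; Grim enemy Blueprint that provides melee, projectile and teleport actions, plus its own movement speeds and ideal combat ranges.
; Attacks route through the BPCAttacks component: a zero-damage forward melee trace and a non-homing projectile with a montage.
; Teleport is a disguised fast flight: it hides the mesh, ignores Pawn collision, attaches a Niagara effect and uses AIMoveTo.
; TeleportEnd restores walking, visibility and collision only on move success; failure is unhandled.
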(event Custom|Teleport
  (params (Location :type Vector))
  (bind _charactermovement (Variables|Character|GetCharacterMovement))
  (if (not (Variables|Default|GetIsTeleporting))
    (Variables|Default|SetIsTeleporting true)
    (Pawn|Components|CharacterMovement|SetMovementMode _charactermovement "MOVE_Flying" 0)
    (Variables|/Script/Engine.CharacterMovementComponent|SetMaxFlySpeed _charactermovement 5e+03)
    (Variables|/Script/Engine.CharacterMovementComponent|SetMaxAcceleration _charactermovement 99999.0)
    (Rendering|SetVisibility (Variables|Character|GetMesh) false true)
    (Collision|SetCollisionResponsetoChannel (Variables|Default|GetCapsuleComponent) "ECC_Pawn" "ECR_Ignore")
    ;[1 1 1] Spawn emitter or niagra effect as needed
    (bind _returnvalue (Niagara|SpawnSystemAttached "/Game/Levels/BlockMesh_Assets/GyzerNiagaraSystem.GyzerNiagaraSystem" (Variables|Character|GetMesh) "None" "0, 0, 0" "0, 0, 0" "KeepRelativeOffset" false))
    (Variables|Default|SetNiagraEffect _returnvalue)
    (AI|AIMoveTo self Location 0 15.0 false
      (:OnSuccess
        (CallFunction|TeleportEnd)))
    (else
      (Utilities|FlowControl|DelayUntilNextTick)
      (Default|CallOnTeleportEnd))))

(event Custom|TeleportEnd
  (bind _charactermovement (Variables|Character|GetCharacterMovement))
  (Components|Movement|StopMovementImmediately _charactermovement)
  (Pawn|Components|CharacterMovement|SetMovementMode _charactermovement "MOVE_Walking" 0)
  (Variables|/Script/Engine.CharacterMovementComponent|SetMaxAcceleration _charactermovement 1.5e+03)
  (Rendering|SetVisibility (Variables|Character|GetMesh) true true)
  (Collision|SetCollisionResponsetoChannel (Variables|Default|GetCapsuleComponent) "ECC_Pawn" "ECR_Block")
  (Variables|Default|SetIsTeleporting false)
  (Utilities|FlowControl|Sequence
    (:then_0
      (bind _niagraeffect (Variables|Default|GetNiagraEffect)
        (:then
          (Components|DestroyComponent _niagraeffect))
        (:else)))
    (:then_1
      (Default|CallOnTeleportEnd))))

(event Custom|MeleeAttack
  (params (AttackTarget :type Actor%20Object%20Reference))
  (bind _returnvalue (Transformation|GetActorLocation))
  (Default|MeleeAttack (Variables|Default|GetBPC_Attacks) _returnvalue (+ _returnvalue (* (Transformation|GetActorForwardVector) 1e+02)) (Utilities|Struct|MakeBPS_EnemyAttackInfo AttackTarget 0 (Utilities|Struct|MakeBPS_DamageInfo 0.0 0.0)) 0.0))

(event Custom|ProjectileAttack
  (params (AttackTarget :type Actor%20Object%20Reference))
  (Default|ProjectileAttack (Variables|Default|GetBPC_Attacks) (Transformation|GetWorldTransform (Variables|Default|GetStartAttack)) false (Utilities|Struct|MakeBPS_EnemyAttackInfo AttackTarget "/Game/Assets/Enemies/Grim/Montage/Grim_Projectile_Montage.Grim_Projectile_Montage" (Utilities|Struct|MakeBPS_DamageInfo 2e+01 0.0 "NewEnumerator2"))))

(event EventBeginPlay
  (|CallParentFunction) ; This node is disabled and will not be called.\nDrag off pins to build functionality.
)

(event Collision|EventActorBeginOverlap
  (params (OtherActor :type Actor%20Object%20Reference)))

(event EventTick
  (params (DeltaSeconds :type Float%20%28single-precision%29)))

(fn ConstructionScript
  (|CallParentFunction))

(fn SetMovementSpeed
  (params (Speed :type BPE_MovementSpeed%20Enum :default "NewEnumerator0"))
  (return (Utilities|Select :Index Speed :NewEnumerator0 0.0 :NewEnumerator1 1.5e+02 :NewEnumerator2 3e+02 :NewEnumerator4 5e+02 :NewEnumerator5 1e+03)))

(fn GetIdealRange
  (return 1e+02 2e+02 5e+02 7e+02))

(fn AttackStart
  (params (AttackTarget :type Actor%20Object%20Reference) (TokensNeeded :type Integer))
  (bind _success (|CallParentFunction AttackTarget TokensNeeded))
  (return _success))