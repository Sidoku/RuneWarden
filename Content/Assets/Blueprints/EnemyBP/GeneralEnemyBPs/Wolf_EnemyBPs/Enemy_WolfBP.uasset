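; Wolf enemy Blueprint that supplies the species-specific health, attacks and ideal combat ranges.
; Bite and leap attack events pack montage and damage into attack info for the shared attacks component, with a short forward trace for the bite and an arced jump for the leap.
; Construction sets health on the damage system component, and an event passes the head-turn flag to the wolf Animation Blueprint.
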(event Custom|MeleeAttack
  (params (AttackTarget :type Actor%20Object%20Reference))
  (bind _returnvalue (Transformation|GetActorLocation))
  ;[1 1 1] Melee Attack
  (Default|MeleeAttack (Variables|Default|GetBPC_Attacks) _returnvalue (+ _returnvalue (* (Transformation|GetActorForwardVector) 1e+02)) (Utilities|Struct|MakeBPS_EnemyAttackInfo AttackTarget "/Game/Assets/Enemies/Wolf/Montages/Wolf_Bite_Montage.Wolf_Bite_Montage" (Utilities|Struct|MakeBPS_DamageInfo 2e+01 0.0 "NewEnumerator1")) 5e+01))

(event Custom|LeapAttack
  (params (AttackTarget :type Actor%20Object%20Reference))
  ;[1 1 1] Leap Attack
  (Default|LeapAttack (Variables|Default|GetBPC_Attacks) (Utilities|Struct|MakeBPS_EnemyAttackInfo AttackTarget "/Game/Assets/Enemies/Wolf/Montages/Wolf_Leap_Montage.Wolf_Leap_Montage" (Utilities|Struct|MakeBPS_DamageInfo 3e+01 0.0 "NewEnumerator1")) 0.7))

(event EventBeginPlay
  (|CallParentFunction) ; This node is disabled and will not be called.\nDrag off pins to build functionality.
)

(event Collision|EventActorBeginOverlap
  (params (OtherActor :type Actor%20Object%20Reference)))

(event EventTick
  (params (DeltaSeconds :type Float%20%28single-precision%29)))

(event EventSetCanTurnHead
  (params (CanTurnHead :type Boolean))
  (bind _aswolf_abp (Utilities|Casting|CastToWolf_ABP (Components|SkeletalMesh|GetAnimInstance (Variables|Character|GetMesh))))
  (Variables|/Game/Assets/Enemies/Wolf/Wolf_ABP.Wolf_ABP_C|SetCanTurnHead _aswolf_abp CanTurnHead))

(fn ConstructionScript
  (bind _bpc_damagesystem (Variables|Default|GetBPC_DamageSystem))
  (|CallParentFunction)
  (Variables|/Game/Assets/DamageSystem/BPC_DamageSystem.BPC_DamageSystem_C|SetMaxHealth _bpc_damagesystem 1e+02)
  (Variables|/Game/Assets/DamageSystem/BPC_DamageSystem.BPC_DamageSystem_C|SetCurrentHealth _bpc_damagesystem 1e+02))

(fn GetIdealRange
  (return 1.5e+02 1.6e+03 2.8e+03 4.5e+03))