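; Statue enemy Blueprint, a child of a base enemy, that fights with a sword using melee and area attacks.
; On BeginPlay it runs the parent logic and snaps the sword to the EquipSword socket.
; MeleeAttack and AOEAttack hand montage and damage info to the BPCAttacks component, with melee tracing a short sphere ahead of the statue.
; An unconnected node for unhiding the sword never runs.
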(event Custom|MeleeAttack
  (params (AttackTarget :type Actor%20Object%20Reference))
  (bind _returnvalue (Transformation|GetActorLocation))
  ;[1 1 1] Melee Attack
  (Default|MeleeAttack (Variables|Default|GetBPC_Attacks) _returnvalue (+ _returnvalue (* (Transformation|GetActorForwardVector) 1e+02)) (Utilities|Struct|MakeBPS_EnemyAttackInfo AttackTarget "/Game/Assets/Enemies/Statue/Montage/StatueCombo1_Montage.StatueCombo1_Montage" (Utilities|Struct|MakeBPS_DamageInfo 2e+01 0.0 "NewEnumerator1")) 5e+01))

(event Custom|AOE%20Attack
  (params (AttackTarget :type Actor%20Object%20Reference))
  (Default|TestAOEAttack (Variables|Default|GetBPC_Attacks) (Utilities|Struct|MakeBPS_EnemyAttackInfo AttackTarget "/Game/Assets/Enemies/Statue/Montage/StatueAoE_Montage.StatueAoE_Montage" (Utilities|Struct|MakeBPS_DamageInfo 2e+01 0.0 "NewEnumerator1"))))

(event EventBeginPlay
  ;[0.15 0.15 0.15 0.5] Equip Sword
  (|CallParentFunction)
  (Transformation|AttachComponentToComponent (Variables|Default|GetSword) 0 "EquipSword" "SnapToTarget" "SnapToTarget" "SnapToTarget" true))

(fn ConstructionScript
  (|CallParentFunction))