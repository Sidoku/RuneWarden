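; One-shot enemy spawner variant that starts a combat encounter when the player enters its box holding one or two keys.
; It briefly halts the player, spawns a combat zone and starts combat music, then after a portal delay spawns player-facing enemies.
; Key count selects the enemy set, with two keys also overriding spawn count, and a MultiGate cycles four spawn points.
; Enemies receive a spawner reference, and DeathSpawnCount removes zone and spawner and stops music once all die.
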(event OnComponentBeginOverlap(Box)
  (params (OverlappedComponent :type Primitive%20Component%20Object%20Reference) (OtherActor :type Actor%20Object%20Reference) (OtherComp :type Primitive%20Component%20Object%20Reference) (OtherBodyIndex :type Integer) (bFromSweep :type Boolean) (SweepResult :type Hit%20Result%20Structure%20%28by%20ref%29))
  (bind _returnvalue (Game|GetPlayerCharacter 0))
  (bind _as_bp_game_instance (Variables|Default|GetAs%20BP%20Game%20Instance))
  (bind _as_bp_game_instance_2 (Variables|Default|GetAs%20BP%20Game%20Instance))
  (bind _portaltimer (Variables|Default|GetPortalTimer))
  (bind _key_count (Variables|/Game/GameState/BP_GameInstance.BP_GameInstance_C|GetKey%20Count _as_bp_game_instance))
  (bind _charactermovement (Variables|/Script/Engine.Character|GetCharacterMovement _returnvalue))
  (bind _key_count_2 (Variables|/Game/GameState/BP_GameInstance.BP_GameInstance_C|GetKey%20Count _as_bp_game_instance_2))
  ;[1 0.04388 0.1636] Spawner Code
  (Utilities|Casting|CastToPlayerCharacterBP OtherActor)
  (if (== _key_count_2 1)
    (Utilities|FlowControl|DoOnce false :!label _label
      (:Completed
        (Utilities|FlowControl|Sequence
          (:then_0
            ;[1 0.1087 0.7842] Combat Zone
            (Pawn|Components|CharacterMovement|SetMovementMode _charactermovement "MOVE_None" 0)
            (Utilities|FlowControl|Delay 0.5)
            (bind _returnvalue_2 (Game|SpawnActorfromClass "/Game/Levels/BlockMesh_Assets/BP_CombatZone.BP_CombatZone_C" (Math|Transform|MakeTransform (Transformation|GetWorldLocation (Variables|Default|GetPortal%20Spawn%20Point)) "0, 0, 0" (Variables|Default|GetCombatZoneSize)) "Undefined" "MultiplyWithRoot" 0 0))
            (Pawn|Components|CharacterMovement|SetMovementMode _charactermovement "MOVE_Walking" 0)
            (bind _returnvalue_3 (Actor|GetActorOfClass (Variables|Default|GetMusicActor%20Ref)))
            (Class|BPIGeneralEnemy|CombatStart(Message) _returnvalue_3))
          (:then_1
            (Utilities|FlowControl|Delay _portaltimer)
            (if (== (Variables|Default|GetSpawn%20Count) 1)
              (Variables|Default|SetOffset%20Spawn%20Enemy 0.0)
              (for _index (range 0 (- (Variables|Default|GetSpawn%20Count) 1)) :!label _label_2
                (if (== _key_count 2)
                  (Utilities|FlowControl|MultiGate false true 0
                    (:Out%200
                      (Variables|Default|SetEnemyRef (Variables|Default|GetVariation1))
                      (Variables|Default|SetSpawn%20Transform%20Location (Transformation|GetWorldLocation (Variables|Default|GetSpawnPoint))))
                    (:Out%201
                      (Variables|Default|SetEnemyRef (Variables|Default|GetVariation2))
                      (Variables|Default|SetSpawn%20Transform%20Location (Transformation|GetWorldLocation (Variables|Default|GetSpawnPoint1))))
                    (:Out%202
                      (Variables|Default|SetEnemyRef (Variables|Default|GetVariation3))
                      (Variables|Default|SetSpawn%20Transform%20Location (Transformation|GetWorldLocation (Variables|Default|GetSpawnPoint2))))
                    (:Out%203
                      (Variables|Default|SetEnemyRef (Variables|Default|GetVariation4))
                      (Variables|Default|SetSpawn%20Transform%20Location (Transformation|GetWorldLocation (Variables|Default|GetSpawnPoint3)))))
                  (bind _returnvalue_4 (Game|SpawnActorfromClass (Variables|Default|GetEnemyRef) (Math|Transform|MakeTransform (Variables|Default|GetSpawn%20Transform%20Location) (Math|Rotator|MakeRotator (.Roll (Math|Rotator|BreakRotator (Math|Rotator|FindLookatRotation (Variables|Default|GetSpawn%20Transform%20Location) (Transformation|GetActorLocation (Game|GetPlayerCharacter 0))))) 0.0 (.Yaw (Math|Rotator|BreakRotator (Math|Rotator|FindLookatRotation (Variables|Default|GetSpawn%20Transform%20Location) (Transformation|GetActorLocation (Game|GetPlayerCharacter 0)))))) "1.000000,1.000000,1.000000") "AdjustIfPossibleButAlwaysSpawn" "MultiplyWithRoot" 0 0 :!label _label_3))
                  (bind _asenemy_bp (Utilities|Casting|CastToEnemyBP _returnvalue_4))
                  (Variables|/Game/Assets/Blueprints/EnemyBP/GeneralEnemyBPs/EnemyBP.EnemyBP_C|SetBPSpawnerRef _asenemy_bp self)
                  (elif (== _key_count 1)
                    (Utilities|FlowControl|MultiGate false true 0
                      (:Out%200
                        (Variables|Default|SetEnemyRef (Variables|Default|GetKey1enemy))
                        (Variables|Default|SetSpawn%20Transform%20Location (Transformation|GetWorldLocation (Variables|Default|GetSpawnPoint)))
                        (goto _label_3))
                      (:Out%201
                        (Variables|Default|SetEnemyRef (Variables|Default|GetKey1enemy2))
                        (Variables|Default|SetSpawn%20Transform%20Location (Transformation|GetWorldLocation (Variables|Default|GetSpawnPoint1)))
                        (goto _label_3))
                      (:Out%202
                        (Variables|Default|SetEnemyRef (Variables|Default|GetKey1Enemy3))
                        (Variables|Default|SetSpawn%20Transform%20Location (Transformation|GetWorldLocation (Variables|Default|GetSpawnPoint2)))
                        (goto _label_3))
                      (:Out%203
                        (Variables|Default|SetEnemyRef (Variables|Default|GetKey1Enemy4))
                        (Variables|Default|SetSpawn%20Transform%20Location (Transformation|GetWorldLocation (Variables|Default|GetSpawnPoint3)))
                        (goto _label_3))))))))
          (:then_2
            (Utilities|FlowControl|Delay _portaltimer)
            (if (== (Variables|Default|GetSpawn%20Count) 2)
              (Variables|Default|SetOffset%20Spawn%20Enemy 0.5)
              (goto _label_2)))
          (:then_3
            (Utilities|FlowControl|Delay _portaltimer)
            (if (== (Variables|Default|GetSpawn%20Count) 3)
              (Variables|Default|SetOffset%20Spawn%20Enemy 1.0)
              (goto _label_2)))
          (:then_4
            (Utilities|FlowControl|Delay _portaltimer)
            (if (== (Variables|Default|GetSpawn%20Count) 4)
              (Variables|Default|SetOffset%20Spawn%20Enemy 1.5)
              (goto _label_2))))))
    (elif (== _key_count_2 2)
      (Variables|Default|SetSpawn%20Count (Variables|Default|GetVariationSpawnCount))
      (goto _label))))

(event EventDeathSpawnCount
  (bind _deathcounter (Variables|Default|GetDeathCounter))
  (bind _result (Math|Integer|IncrementInt _deathcounter)
    (:%20%20
      (if (== _result (Variables|Default|GetSpawn%20Count))
        ;[1 1 1] Frankie spawner collision zone section
        (Development|PrintString "All spawned enemies are dead")
        ;[1 1 1] Destory spawner and combat sphere
        (Actor|DestroyActor (stale OnComponentBeginOverlap(Box) _returnvalue_2))
        (Class|BPIGeneralEnemy|CombatStop(Message) (stale OnComponentBeginOverlap(Box) _returnvalue_3))
        (Actor|DestroyActor)
        (else
          (Development|PrintString (Utilities|String|ToString(Integer) _deathcounter)))))))

(event Collision|EventActorBeginOverlap
  (params (OtherActor :type Actor%20Object%20Reference))
  ;[1 0.04388 0.1636] Spawner Code
)

(event EventTick
  (params (DeltaSeconds :type Float%20%28single-precision%29))
  ;[1 0.04388 0.1636] Spawner Code
)

(event EventBeginPlay
  (|CallParentFunction))

(fn ConstructionScript
  (|CallParentFunction))