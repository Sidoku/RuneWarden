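; Beast enemy Blueprint, a child enemy class that defines the creature's two melee slashes, a leap attack and its ideal combat ranges.
; Each attack event packs target, montage and damage into an attack info struct for BPCAttacks, with slashes tracing just ahead and the leap following a sound and short delay.
; GetIdealRange supplies the melee and ranged distance bands.
; A hit-stop call is present but unconnected.
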(event Custom|Melee%20Attack%202
  (params (AttackTarget :type Actor%20Object%20Reference))
  (bind _returnvalue (Transformation|GetActorLocation))
  ;[1 1 1] Melee Attack 2
  (Default|MeleeAttack (Variables|Default|GetBPC_Attacks) _returnvalue (+ _returnvalue (* (Transformation|GetActorForwardVector) 1e+02)) (Utilities|Struct|MakeBPS_EnemyAttackInfo AttackTarget "/Game/Assets/Enemies/Beast/Montage/Beast_Slash_2_Montage.Beast_Slash_2_Montage" (Utilities|Struct|MakeBPS_DamageInfo 5.0 0.0 "NewEnumerator1")) 1e+02))

(event Custom|Leap%20Attack
  (params (AttackTarget :type Actor%20Object%20Reference))
  ;[1 1 1] Leap Attack
  (Audio|PlaySoundatLocation "/Game/Assets/Sounds/Beast/Beast_Leap.Beast_Leap" (Transformation|GetActorLocation (Components|GetOwner)) "0, 0, 0" 1.0 1.0 0.0 0 0 0 0)
  (Utilities|FlowControl|Delay 0.3)
  (Default|LeapAttack (Variables|Default|GetBPC_Attacks) (Utilities|Struct|MakeBPS_EnemyAttackInfo AttackTarget "/Game/Assets/Enemies/Beast/Montage/ForwardLeap_Montage.ForwardLeap_Montage" (Utilities|Struct|MakeBPS_DamageInfo 1e+01 0.0 "NewEnumerator1")) 0.5))

(event Custom|Melee%20Attack
  (params (AttackTarget :type Actor%20Object%20Reference))
  (bind _returnvalue (Transformation|GetActorLocation))
  ;[1 1 1] Melee Attack
  (Default|MeleeAttack (Variables|Default|GetBPC_Attacks) _returnvalue (+ _returnvalue (* (Transformation|GetActorForwardVector) 1e+02)) (Utilities|Struct|MakeBPS_EnemyAttackInfo AttackTarget "/Game/Assets/Enemies/Beast/Montage/Beast_Slash_1_Montage.Beast_Slash_1_Montage" (Utilities|Struct|MakeBPS_DamageInfo 5.0 0.0 "NewEnumerator1")) 1e+02))

(event EventBeginPlay
  (|CallParentFunction))

(fn ConstructionScript
  (|CallParentFunction))

(fn GetIdealRange
  (return 2e+02 1.6e+03 2.8e+03 4.5e+03))