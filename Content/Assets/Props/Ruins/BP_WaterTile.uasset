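; BP_WaterTile is a water tile prop in the Ruins set that slides between StartLocation and DesiredLocation.
; Tick feeds a four-second Delay, acting as a repeating trigger for RunSidetosidemovement.
; That event's FlipFlop alternates two timelines, MoveLeft and Timeline, each lerping the actor's location between the same points without sweep.
; The graph never sets either location, and a looping timer setup is left unconnected.
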(event Custom|Run%20Side%20to%20side%20movement
  (Utilities|FlowControl|FlipFlop
    (:A
      (bind _newtrack_0 (Timeline|Move%20Left PlayFromStart)
        (:Update
          (Transformation|SetActorLocation (Math|Vector|Lerp(Vector) (Variables|Default|GetStart%20Location) (Variables|Default|GetDesired%20location) _newtrack_0) false false))))
    (:B
      (bind _newtrack_0_2 (Timeline|Timeline PlayFromStart)
        (:Update
          (Transformation|SetActorLocation (Math|Vector|Lerp(Vector) (Variables|Default|GetStart%20Location) (Variables|Default|GetDesired%20location) _newtrack_0_2) false false))))))

(event EventBeginPlay)

(event Collision|EventActorBeginOverlap
  (params (OtherActor :type Actor%20Object%20Reference)))

(event EventTick
  (params (DeltaSeconds :type Float%20%28single-precision%29))
  (Utilities|FlowControl|Delay 4.0)
  (CallFunction|RunSidetoSideMovement))

(fn ConstructionScript)