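; BP_SpiritLight is a prop that travels back and forth along the PatrolRoute spline of a BP_LightSpline found at BeginPlay.
; Tick plays or reverses a timeline based on SplineBool, and the timeline's alpha sets the actor's world location along the spline's length.
; On finish, a FlipFlop toggles SplineBool and prints debug text.
; Attack, range and speed functions are empty stubs, and some unconnected experimental nodes remain.
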(event Custom|Run%20Spline)

(event Custom|Flip
  (Utilities|FlowControl|FlipFlop
    (:A
      (Variables|Default|SetSplineBool false)
      (Development|PrintString "Finished Spline"))
    (:B
      (Variables|Default|SetSplineBool true)
      (Development|PrintString "Finished Spline2"))))

(event EventBeginPlay
  (bind _returnvalue (Actor|GetActorOfClass "/Game/Assets/Blueprints/BP_LightSpline.BP_LightSpline_C")))

(event EventTick
  (params (DeltaSeconds :type Float%20%28single-precision%29))
  (if (Variables|Default|GetSplineBool)
    (bind _newtrack_0 (Timeline|Timeline Play)
      (:Update
        (Transformation|SetActorLocation (Spline|GetLocationatDistanceAlongSpline (Variables|/Game/Assets/Blueprints/BP_LightSpline.BP_LightSpline_C|GetPatrolRoute (stale EventBeginPlay _returnvalue)) (Math|Float|Lerp (Variables|Default|GetA) (Spline|GetSplineLength (Variables|/Game/Assets/Blueprints/BP_LightSpline.BP_LightSpline_C|GetPatrolRoute (stale EventBeginPlay _returnvalue))) _newtrack_0) "World") false false))
      (:Finished
        (CallFunction|Flip)))
    (else
      (Timeline|Timeline Reverse))))

(fn ConstructionScript)

(fn AttackStart
  (params (AttackTarget :type Actor%20Object%20Reference) (TokensNeeded :type Integer))
  (return false))

(fn GetIdealRange
  (return 0.0 0.0 0.0 0.0))

(fn SetMovementSpeed
  (params (Speed :type BPE_MovementSpeed%20Enum :default "NewEnumerator0"))
  (return 0.0))

(fn GetPatrolRoute
  (return (Variables|Default|GetPatrol%20Route)))