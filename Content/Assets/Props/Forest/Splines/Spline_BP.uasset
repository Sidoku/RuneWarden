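; Spline prop Blueprint that builds a run of spline mesh components from its Spline when constructed.
; The construction script adds one component per SectionLength step of spline length, each using SplineMesh, with optional section length scaling from actor X scale.
; The MustBeFullLengthMeshes branch creates nothing, and the shown graph never sets the segments' start, end or tangents.
; The event graph holds no active logic.
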(event EventBeginPlay)

(event Collision|EventActorBeginOverlap
  (params (OtherActor :type Actor%20Object%20Reference)))

(event EventTick
  (params (DeltaSeconds :type Float%20%28single-precision%29)))

(fn ConstructionScript
  (if (Variables|Default|GetAllow%20Scaling?)
    ;[1 1 1] Scale Spline
    (Variables|Default|SetSectionLength (* (.x (Transformation|GetActorScale3D)) 1e+02)))
  (if (Variables|Default|GetMust%20be%20Full%20Length%20Meshes?)
    (for _index (range 0 0)
      _)
    (else
      ;[1 1 1] Amount of Spline Meshes
      (for _index_2 (range 0 (Math|Float|Truncate (/ (Spline|GetSplineLength (Variables|Default|GetSpline)) (Variables|Default|GetSectionLength))))
        (Variables|Default|SetIndex _index_2)
        (bind _returnvalue (AddComponent|AddSplineMeshComponent false))
        (Components|StaticMesh|SetStaticMesh _returnvalue (Variables|Default|GetSpline%20Mesh))))))