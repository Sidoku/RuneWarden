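; Music controller Blueprint for the volcano area, switching one audio component between intro, loop and combat tracks.
; BeginPlay fades in the intro, then after a 51-second delay moves to the loop if HitsCollisionBeforeTimerStop is still true.
; CombatStart clears that flag and plays combat music; CombatStop restores the loop.
; Each switch calls FadeOut, SetSound and FadeIn without waiting; Block, KnockBack, Stagger and Target are stubs returning false.
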(event EventBeginPlay
  (bind _audiocomponent (Variables|Components|GetAudioComponent))
  (Audio|Components|Audio|SetSound _audiocomponent "/Game/Assets/Music/VolcanoBeginning.VolcanoBeginning")
  (Audio|Components|Audio|FadeIn _audiocomponent 2.0 1.0 0.0 "Linear" :!class /Script/Engine.AudioComponent)
  (Utilities|FlowControl|Delay 51.0)
  (if (Variables|Default|GetHits%20collision%20before%20timer%20stop)
    (Audio|Components|Audio|FadeOut _audiocomponent 2.0 0.0 "Linear" :!class /Script/Engine.AudioComponent)
    (Audio|Components|Audio|SetSound _audiocomponent "/Game/Assets/Music/VolcanoLoop.VolcanoLoop")
    (Audio|Components|Audio|FadeIn _audiocomponent 2.0 1.0 0.0 "Linear" :!class /Script/Engine.AudioComponent)))

(event EventTick
  (params (DeltaSeconds :type Float%20%28single-precision%29)))

(event EventCombatStart
  (bind _audiocomponent (Variables|Components|GetAudioComponent))
  (Variables|Default|SetHits%20collision%20before%20timer%20stop false)
  (Audio|Components|Audio|FadeOut _audiocomponent 2.0 0.0 "Linear" :!class /Script/Engine.AudioComponent)
  ;[0.15 0.15 0.15 0.5] Combat Sound
  (Audio|Components|Audio|SetSound _audiocomponent "/Game/Assets/Music/VolcanoCombat.VolcanoCombat")
  (Audio|Components|Audio|FadeIn _audiocomponent 2.0 1.0 0.0 "Linear" :!class /Script/Engine.AudioComponent))

(event EventCombatStop
  (bind _audiocomponent (Variables|Components|GetAudioComponent))
  (Audio|Components|Audio|FadeOut _audiocomponent 2.0 0.0 "Linear" :!class /Script/Engine.AudioComponent)
  (Audio|Components|Audio|SetSound _audiocomponent "/Game/Assets/Music/VolcanoLoop.VolcanoLoop")
  (Audio|Components|Audio|FadeIn _audiocomponent 2.0 1.0 0.0 "Linear" :!class /Script/Engine.AudioComponent))

(fn ConstructionScript)

(fn Block
  (params (CanBlock? :type Boolean) (BlockDamage :type Float%20%28double-precision%29) (BlockBroken? :type Boolean))
  (return false false))

(fn KnockBack
  (params (CanKnockBack? :type Boolean) (KnockBackDistance :type Float%20%28double-precision%29))
  (return false))

(fn Stagger
  (params (CanStagger? :type Boolean))
  (return false))

(fn Target
  (params (CanTarget? :type Boolean) (TargetDistance :type Float%20%28double-precision%29))
  (return false))