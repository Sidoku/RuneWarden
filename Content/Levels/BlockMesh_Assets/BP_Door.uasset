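; BP_Door is a double sliding door that opens and closes as things enter and leave its OpenTrigger.
; BeginPlay caches each panel's closed position and a target offset in opposite directions along world X; separate timelines lerp the panels between them, always playing from start.
; A separate GlowTrigger swaps both panels to a dynamic emissive material on overlap and restores the wall tile material on exit.
; Sound nodes are present but unconnected.
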(event OnComponentBeginOverlap(OpenTrigger)
  (params (OverlappedComponent :type Primitive%20Component%20Object%20Reference) (OtherActor :type Actor%20Object%20Reference) (OtherComp :type Primitive%20Component%20Object%20Reference) (OtherBodyIndex :type Integer) (bFromSweep :type Boolean) (SweepResult :type Hit%20Result%20Structure%20%28by%20ref%29))
  (Utilities|FlowControl|Sequence
    (:then_0
      (bind _newtrack_2 (Timeline|Move%20Door PlayFromStart)
        (:Update
          (Transformation|SetWorldLocation (Variables|Default|GetDoor1) (Math|Vector|Lerp(Vector) (Variables|Default|GetDoor1Location) (Variables|Default|GetDoor1Target%20location) _newtrack_2) false false))))
    (:then_1
      (bind _newtrack_2_2 (Timeline|Timeline PlayFromStart)
        (:Update
          (Transformation|SetWorldLocation (Variables|Default|GetDoor2) (Math|Vector|Lerp(Vector) (Variables|Default|GetDoor2Location) (Variables|Default|GetDoor2Target%20location) _newtrack_2_2) false false))))))

(event OnComponentBeginOverlap(GlowTrigger)
  (params (OverlappedComponent :type Primitive%20Component%20Object%20Reference) (OtherActor :type Actor%20Object%20Reference) (OtherComp :type Primitive%20Component%20Object%20Reference) (OtherBodyIndex :type Integer) (bFromSweep :type Boolean) (SweepResult :type Hit%20Result%20Structure%20%28by%20ref%29))
  (bind _returnvalue (Rendering|Material|CreateDynamicMaterialInstance "/Game/Assets/Materials/MaterialInstances/MI_Ruins/MI_WallTileEmissive.MI_WallTileEmissive" "None" "None" :!class /Script/Engine.KismetMaterialLibrary))
  (Rendering|Material|SetMaterial (Variables|Default|GetDoor2) 0 _returnvalue))

(event OnComponentEndOverlap(OpenTrigger)
  (params (OverlappedComponent :type Primitive%20Component%20Object%20Reference) (OtherActor :type Actor%20Object%20Reference) (OtherComp :type Primitive%20Component%20Object%20Reference) (OtherBodyIndex :type Integer))
  (Utilities|FlowControl|Sequence
    (:then_0
      (bind _newtrack_2 (Timeline|Timeline_0 PlayFromStart)
        (:Update
          (Transformation|SetWorldLocation (Variables|Default|GetDoor1) (Math|Vector|Lerp(Vector) (Variables|Default|GetDoor1Target%20location) (Variables|Default|GetDoor1Location) _newtrack_2) false false))))
    (:then_1
      (bind _newtrack_2_2 (Timeline|Timeline_1 PlayFromStart)
        (:Update
          (Transformation|SetWorldLocation (Variables|Default|GetDoor2) (Math|Vector|Lerp(Vector) (Variables|Default|GetDoor2Target%20location) (Variables|Default|GetDoor2Location) _newtrack_2_2) false false))))))

(event OnComponentEndOverlap(GlowTrigger)
  (params (OverlappedComponent :type Primitive%20Component%20Object%20Reference) (OtherActor :type Actor%20Object%20Reference) (OtherComp :type Primitive%20Component%20Object%20Reference) (OtherBodyIndex :type Integer))
  (Rendering|Material|SetMaterial (Variables|Default|GetDoor1) 0 "/Game/Assets/Materials/MaterialInstances/MI_Ruins/MI_WallTile1.MI_WallTile1"))

(event EventBeginPlay
  (bind _door1 (Variables|Default|GetDoor1))
  (bind _door2 (Variables|Default|GetDoor2))
  (bind _returnvalue (Transformation|GetWorldLocation _door2))
  (bind _returnvalue_2 (Transformation|GetWorldLocation _door1))
  (Variables|Default|SetDoor1Location _returnvalue_2)
  (Variables|Default|SetDoor1Target%20location (+ _returnvalue_2 "60.000000,0.000000,0.000000"))
  (Variables|Default|SetDoor2Location _returnvalue)
  (Variables|Default|SetDoor2Target%20location (- _returnvalue "60.000000,0.000000,0.000000")))

(event Collision|EventActorBeginOverlap
  (params (OtherActor :type Actor%20Object%20Reference)))

(event EventTick
  (params (DeltaSeconds :type Float%20%28single-precision%29)))

(fn ConstructionScript)