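; Volcano portal door that opens when the player character enters its Box trigger and closes when they leave.
; BeginPlay caches the relative start positions of four corner panels and a center piece.
; Separate timelines per piece and direction drive relative-location lerps.
; Opening blends from each piece's current position toward its target, while closing always starts from the fully open target, even if opening was interrupted.
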(event OnComponentBeginOverlap(Box)
  (params (OverlappedComponent :type Primitive%20Component%20Object%20Reference) (OtherActor :type Actor%20Object%20Reference) (OtherComp :type Primitive%20Component%20Object%20Reference) (OtherBodyIndex :type Integer) (bFromSweep :type Boolean) (SweepResult :type Hit%20Result%20Structure%20%28by%20ref%29))
  (Utilities|Casting|CastToPlayerCharacterBP OtherActor)
  (CallFunction|OpenDoor))

(event OnComponentEndOverlap(Box)
  (params (OverlappedComponent :type Primitive%20Component%20Object%20Reference) (OtherActor :type Actor%20Object%20Reference) (OtherComp :type Primitive%20Component%20Object%20Reference) (OtherBodyIndex :type Integer))
  (Utilities|Casting|CastToPlayerCharacterBP OtherActor)
  (CallFunction|DoorClose))

(event Custom|Open%20Door
  (bind _center (Variables|Default|GetCenter))
  (bind _dlu_ (Variables|Default|GetDLU_))
  (bind _dld_ (Variables|Default|GetDLD_))
  (bind _dru_ (Variables|Default|GetDRU_))
  (bind _drd_ (Variables|Default|GetDRD_))
  (Utilities|FlowControl|Sequence
    (:then_0
      (bind _doorleftup (Timeline|DoorLeftUP PlayFromStart)
        (:Update
          (Transformation|SetRelativeLocation _dlu_ (Math|Vector|Lerp(Vector) (Variables|/Script/Engine.SceneComponent|GetRelativeLocation _dlu_) (Variables|Default|GetDLU) _doorleftup) false false))))
    (:then_1
      (bind _doorleftup_2 (Timeline|DoorLeftDown PlayFromStart)
        (:Update
          (Transformation|SetRelativeLocation _dld_ (Math|Vector|Lerp(Vector) (Variables|/Script/Engine.SceneComponent|GetRelativeLocation _dld_) (Variables|Default|GetDLD) _doorleftup_2) false false))))
    (:then_2
      (bind _doorleftup_3 (Timeline|DoorRight%20Up PlayFromStart)
        (:Update
          (Transformation|SetRelativeLocation _dru_ (Math|Vector|Lerp(Vector) (Variables|/Script/Engine.SceneComponent|GetRelativeLocation _dru_) (Variables|Default|GetDRU) _doorleftup_3) false false))))
    (:then_3
      (bind _doorleftup_4 (Timeline|Door%20Right%20Down PlayFromStart)
        (:Update
          (Transformation|SetRelativeLocation _drd_ (Math|Vector|Lerp(Vector) (Variables|/Script/Engine.SceneComponent|GetRelativeLocation _drd_) (Variables|Default|GetDRD) _doorleftup_4) false false))))
    (:then_4
      (bind _doorleftup_5 (Timeline|Timeline_3 PlayFromStart)
        (:Update
          (Transformation|SetRelativeLocation _center (Math|Vector|Lerp(Vector) (Variables|/Script/Engine.SceneComponent|GetRelativeLocation _center) (Variables|Default|GetCenterEnd) _doorleftup_5) false false))))))

(event Custom|Door%20Close
  (Utilities|FlowControl|Sequence
    (:then_0
      (bind _doorleftup (Timeline|Timeline PlayFromStart)
        (:Update
          (Transformation|SetRelativeLocation (Variables|Default|GetDLU_) (Math|Vector|Lerp(Vector) (Variables|Default|GetDLU) (Variables|Default|GetDLU_START) _doorleftup) false false))))
    (:then_1
      (bind _doorleftup_2 (Timeline|Timeline_0 PlayFromStart)
        (:Update
          (Transformation|SetRelativeLocation (Variables|Default|GetDLD_) (Math|Vector|Lerp(Vector) (Variables|Default|GetDLD) (Variables|Default|GetDLD_START) _doorleftup_2) false false))))
    (:then_2
      (bind _doorleftup_3 (Timeline|Timeline_1 PlayFromStart)
        (:Update
          (Transformation|SetRelativeLocation (Variables|Default|GetDRU_) (Math|Vector|Lerp(Vector) (Variables|Default|GetDRU) (Variables|Default|GetDRU_START) _doorleftup_3) false false))))
    (:then_3
      (bind _doorleftup_4 (Timeline|Timeline_2 PlayFromStart)
        (:Update
          (Transformation|SetRelativeLocation (Variables|Default|GetDRD_) (Math|Vector|Lerp(Vector) (Variables|Default|GetDRD) (Variables|Default|GetDRD_START) _doorleftup_4) false false))))
    (:then_4
      (bind _doorleftup_5 (Timeline|Timeline_4 PlayFromStart)
        (:Update
          (Transformation|SetRelativeLocation (Variables|Default|GetCenter) (Math|Vector|Lerp(Vector) (Variables|Default|GetCenterEnd) (Variables|Default|GetCenterSTART) _doorleftup_5) false false))))))

(event EventBeginPlay
  ;[1 1 1] Preset Start Location
  (Variables|Default|SetDLU_START (Variables|/Script/Engine.SceneComponent|GetRelativeLocation (Variables|Default|GetDLU_)))
  (Variables|Default|SetDLD_START (Variables|/Script/Engine.SceneComponent|GetRelativeLocation (Variables|Default|GetDLD_)))
  (Variables|Default|SetDRU_START (Variables|/Script/Engine.SceneComponent|GetRelativeLocation (Variables|Default|GetDRU_)))
  (Variables|Default|SetDRD_START (Variables|/Script/Engine.SceneComponent|GetRelativeLocation (Variables|Default|GetDRD_)))
  (Variables|Default|SetCenterSTART (Variables|/Script/Engine.SceneComponent|GetRelativeLocation (Variables|Default|GetCenter))))

(event Collision|EventActorBeginOverlap
  (params (OtherActor :type Actor%20Object%20Reference)))

(event EventTick
  (params (DeltaSeconds :type Float%20%28single-precision%29)))

(fn ConstructionScript)