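; Left hub door that slides open when the player enters its Box trigger and closes when the player leaves.
; Overlap begin and end each play a 2D sound and restart their own timeline from the start.
; Each timeline moves the whole actor toward the open or start location, lerping from the mesh's current world location every update rather than from a cached origin.
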(event OnComponentBeginOverlap(Box)
  (params (OverlappedComponent :type Primitive%20Component%20Object%20Reference) (OtherActor :type Actor%20Object%20Reference) (OtherComp :type Primitive%20Component%20Object%20Reference) (OtherBodyIndex :type Integer) (bFromSweep :type Boolean) (SweepResult :type Hit%20Result%20Structure%20%28by%20ref%29))
  (Utilities|Casting|CastToPlayerCharacterBP OtherActor)
  ;[1 1 1] Sound
  (Audio|PlaySound2D "/Engine/VREditor/Sounds/UI/Scaling_Up.Scaling_Up" 1.0 1.0 0.0 0 0)
  (bind _opendoor (Timeline|OpenLeftDoor PlayFromStart)
    (:Update
      (Transformation|SetActorLocation (Math|Vector|Lerp(Vector) (Transformation|GetWorldLocation (Variables|Debug|GetStaticMeshComponent)) (Variables|Default|GetDoor%20Open%20Location) _opendoor) false false))))

(event OnComponentEndOverlap(Box)
  (params (OverlappedComponent :type Primitive%20Component%20Object%20Reference) (OtherActor :type Actor%20Object%20Reference) (OtherComp :type Primitive%20Component%20Object%20Reference) (OtherBodyIndex :type Integer))
  (Utilities|Casting|CastToPlayerCharacterBP OtherActor)
  ;[1 1 1] Sound
  (Audio|PlaySound2D "/Engine/VREditor/Sounds/UI/Scaling_Down.Scaling_Down" 1.0 1.0 0.0 0 0)
  (bind _opendoor (Timeline|Timeline PlayFromStart)
    (:Update
      (Transformation|SetActorLocation (Math|Vector|Lerp(Vector) (Transformation|GetWorldLocation (Variables|Debug|GetStaticMeshComponent)) (Variables|Default|GetDoor%20Start%20Location) _opendoor) false false))))

(event EventBeginPlay)

(event Collision|EventActorBeginOverlap
  (params (OtherActor :type Actor%20Object%20Reference)))

(event EventTick
  (params (DeltaSeconds :type Float%20%28single-precision%29)))

(fn ConstructionScript)