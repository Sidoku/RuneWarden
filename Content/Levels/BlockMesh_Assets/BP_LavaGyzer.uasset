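; BP_LavaGyzer is a lava geyser level actor that erupts intermittently while the player is inside its box trigger.
; Player overlap opens and enters a Gate, which activates a Niagara effect, waits SpeedOfGyzer, then deactivates it.
; After a random pause it re-enters the Gate, looping until the player leaves the box and closes it.
; The graph only drives the visual effect and applies no damage.
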(event OnComponentBeginOverlap(boxcollision)
  (params (OverlappedComponent :type Primitive%20Component%20Object%20Reference) (OtherActor :type Actor%20Object%20Reference) (OtherComp :type Primitive%20Component%20Object%20Reference) (OtherBodyIndex :type Integer) (bFromSweep :type Boolean) (SweepResult :type Hit%20Result%20Structure%20%28by%20ref%29))
  (Utilities|Casting|CastToPlayerCharacterBP OtherActor)
  (Utilities|FlowControl|Sequence
    (:then_0
      (goto _label Open))
    (:then_1
      (Utilities|FlowControl|Gate true :!label _label
        (:Exit
          (Components|Activation|Activate (Variables|Default|GetNiagara) false)
          (Utilities|FlowControl|Delay (Variables|Default|GetSpeed%20of%20Gyzer))
          (Components|Activation|Deactivate (Variables|Default|GetNiagara))
          (Utilities|FlowControl|Delay (Math|Random|RandomFloatinRange 5.0 8.0))
          (goto _label))))))

(event OnComponentEndOverlap(boxcollision)
  (params (OverlappedComponent :type Primitive%20Component%20Object%20Reference) (OtherActor :type Actor%20Object%20Reference) (OtherComp :type Primitive%20Component%20Object%20Reference) (OtherBodyIndex :type Integer))
  (Utilities|Casting|CastToPlayerCharacterBP OtherActor)
  (Utilities|FlowControl|Gate true) ; enters at Close
)

(event EventBeginPlay)

(event Collision|EventActorBeginOverlap
  (params (OtherActor :type Actor%20Object%20Reference)))

(event EventTick
  (params (DeltaSeconds :type Float%20%28single-precision%29)))

(fn ConstructionScript)