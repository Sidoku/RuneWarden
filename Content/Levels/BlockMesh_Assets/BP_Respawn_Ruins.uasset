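; BP_Respawn_Ruins is a respawn volume for the Ruins level that returns the player to a set point and damages them.
; On BeginPlay it caches the PlayerCharacterBP and the world position of its SpawnLocation component.
; When the player overlaps the Box, it waits briefly, moves them to that position and applies DamageAmount without knockback.
; An unconnected timer and downward ground trace remain in the graph but never run.
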(event OnComponentBeginOverlap(Box)
  (params (OverlappedComponent :type Primitive%20Component%20Object%20Reference) (OtherActor :type Actor%20Object%20Reference) (OtherComp :type Primitive%20Component%20Object%20Reference) (OtherBodyIndex :type Integer) (bFromSweep :type Boolean) (SweepResult :type Hit%20Result%20Structure%20%28by%20ref%29))
  (Utilities|Casting|CastToPlayerCharacterBP OtherActor)
  (Utilities|FlowControl|Delay 0.2)
  (Transformation|SetWorldLocation (Variables|/Script/Engine.Actor|GetRootComponent (Variables|Default|GetPlayerBP)) (Variables|Default|Getrespawn%20location) false false)
  (Default|TakeDamage (Variables|Default|GetPlayerBP) (Utilities|Struct|MakeBPS_DamageInfo (Math|Conversions|ToFloat(Integer) (Variables|Default|GetDamage%20Amount)) 0.0 "NewEnumerator4" "NewEnumerator7" "NewEnumerator2")))

(event EventBeginPlay
  (Utilities|FlowControl|DoOnce false
    (:Completed
      (bind _returnvalue (Actor|GetActorOfClass "/Game/Assets/Blueprints/PlayerBP/PlayerCharacterBP.PlayerCharacterBP_C"))
      (Variables|Default|SetPlayerBP _returnvalue)
      (Variables|Default|Setrespawn%20location (Transformation|GetWorldLocation (Variables|Default|GetSpawn%20Location))))))

(event EventTick
  (params (DeltaSeconds :type Float%20%28single-precision%29)))

(fn ConstructionScript)