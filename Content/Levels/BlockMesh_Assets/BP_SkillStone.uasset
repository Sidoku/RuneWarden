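; BP_SkillStone is a skill stone actor that lets the RuneWarden character trigger the inventory while inside its Box volume.
; Box overlap begin and end set CanTriggerInventory on RuneWarden_BP.
; A RotateStone event spins the stone through RotatingMovement when StoneIsInAir is true and stops it otherwise.
; Float timelines, montage playback and debug prints remain as unconnected logic that never runs, and EnterBox overlaps are empty.
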(event OnComponentBeginOverlap(Box)
  (params (OverlappedComponent :type Primitive%20Component%20Object%20Reference) (OtherActor :type Actor%20Object%20Reference) (OtherComp :type Primitive%20Component%20Object%20Reference) (OtherBodyIndex :type Integer) (bFromSweep :type Boolean) (SweepResult :type Hit%20Result%20Structure%20%28by%20ref%29))
  (bind _asrune_warden_bp (Utilities|Casting|CastToRuneWarden_BP OtherActor))
  (Variables|/Game/Assets/Blueprints/PlayerBP/RuneWarden_BP.RuneWarden_BP_C|SetCanTriggerInventory _asrune_warden_bp true))

(event OnComponentEndOverlap(Box)
  (params (OverlappedComponent :type Primitive%20Component%20Object%20Reference) (OtherActor :type Actor%20Object%20Reference) (OtherComp :type Primitive%20Component%20Object%20Reference) (OtherBodyIndex :type Integer))
  (bind _asrune_warden_bp (Utilities|Casting|CastToRuneWarden_BP OtherActor))
  (Variables|/Game/Assets/Blueprints/PlayerBP/RuneWarden_BP.RuneWarden_BP_C|SetCanTriggerInventory _asrune_warden_bp false))

(event OnComponentBeginOverlap(EnterBox)
  (params (OverlappedComponent :type Primitive%20Component%20Object%20Reference) (OtherActor :type Actor%20Object%20Reference) (OtherComp :type Primitive%20Component%20Object%20Reference) (OtherBodyIndex :type Integer) (bFromSweep :type Boolean) (SweepResult :type Hit%20Result%20Structure%20%28by%20ref%29)))

(event OnComponentEndOverlap(EnterBox)
  (params (OverlappedComponent :type Primitive%20Component%20Object%20Reference) (OtherActor :type Actor%20Object%20Reference) (OtherComp :type Primitive%20Component%20Object%20Reference) (OtherBodyIndex :type Integer)))

(event Custom|Rotate%20Stone
  (bind _rotatingmovement (Variables|Default|GetRotatingMovement))
  (if (Variables|Default|GetStone%20is%20in%20air)
    (Variables|/Script/Engine.RotatingMovementComponent|SetRotationRate _rotatingmovement "0.000000,180.000000,0.000000")
    (else
      (Variables|/Script/Engine.RotatingMovementComponent|SetRotationRate _rotatingmovement "0, 0, 0"))))

(event EventBeginPlay)

(event Collision|EventActorBeginOverlap
  (params (OtherActor :type Actor%20Object%20Reference)))

(event EventTick
  (params (DeltaSeconds :type Float%20%28single-precision%29)))

(fn ConstructionScript)