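; BP_DeadZone is a hazard volume that repeatedly damages a RuneWarden_BP player character standing inside its Box.
; Entering the Box starts a looping half-second timer, which is cleared once an end overlap leaves the Box empty.
; Each tick of the timer re-queries the overlapping actors and sends any RuneWarden_BP a fixed, knockback-free TakeDamageMessage with the zone as dealer.
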(event OnComponentBeginOverlap(Box)
  (params (OverlappedComponent :type Primitive%20Component%20Object%20Reference) (OtherActor :type Actor%20Object%20Reference) (OtherComp :type Primitive%20Component%20Object%20Reference) (OtherBodyIndex :type Integer) (bFromSweep :type Boolean) (SweepResult :type Hit%20Result%20Structure%20%28by%20ref%29))
  (bind _returnvalue (Utilities|Time|SetTimerbyEvent (delegate Custom|Damage) 0.5 true))
  (bind _output_get (Variables|Default|SetTimer _returnvalue)))

(event OnComponentEndOverlap(Box)
  (params (OverlappedComponent :type Primitive%20Component%20Object%20Reference) (OtherActor :type Actor%20Object%20Reference) (OtherComp :type Primitive%20Component%20Object%20Reference) (OtherBodyIndex :type Integer))
  (if (Utilities|Array|IsEmpty (Collision|GetOverlappingActors (Variables|Default|GetBox) 0 :!class /Script/Engine.PrimitiveComponent))
    (Utilities|Time|ClearandInvalidateTimerbyHandle (stale OnComponentBeginOverlap(Box) _output_get))))

(event Custom|Damage
  (for _array_element (Collision|GetOverlappingActors (Variables|Default|GetBox) 0 :!class /Script/Engine.PrimitiveComponent)
    (bind _asplayer_character_bp (Utilities|Casting|CastToRuneWarden_BP _array_element))
    (Class|BPIDamagable|TakeDamage(Message) _asplayer_character_bp (Utilities|Struct|MakeBPS_DamageInfo 5.0 0.0 "NewEnumerator4" "NewEnumerator7" "NewEnumerator2") self)))

(event EventBeginPlay
  (bind _asplayer_character_bp (Utilities|Casting|CastToRuneWarden_BP (Game|Player|GetPlayerPawn 0)))
  (Variables|Default|SetAs%20Player%20Character%20BP _asplayer_character_bp))

(event Collision|EventActorBeginOverlap
  (params (OtherActor :type Actor%20Object%20Reference)))

(event EventTick
  (params (DeltaSeconds :type Float%20%28single-precision%29)))

(fn ConstructionScript)