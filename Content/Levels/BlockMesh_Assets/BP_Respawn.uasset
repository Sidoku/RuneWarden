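; BP_Respawn is a trigger volume that returns the player to a recently recorded ground position and applies damage.
; It caches PlayerCharacterBP on BeginPlay; Tick passes through a five-second Delay, so it periodically saves a downward trace hit as RespawnLocation when the player is not falling.
; Any overlap with the Box, without an actor check, moves the player there after a short delay and deals DamageAmount.
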(event OnComponentBeginOverlap(Box)
  (params (OverlappedComponent :type Primitive%20Component%20Object%20Reference) (OtherActor :type Actor%20Object%20Reference) (OtherComp :type Primitive%20Component%20Object%20Reference) (OtherBodyIndex :type Integer) (bFromSweep :type Boolean) (SweepResult :type Hit%20Result%20Structure%20%28by%20ref%29))
  (Utilities|FlowControl|Delay 0.2)
  (Transformation|SetWorldLocation (Variables|/Script/Engine.Actor|GetRootComponent (Variables|Default|GetPlayerBP)) (Variables|Default|Getrespawn%20location) false false)
  (Default|TakeDamage (Variables|Default|GetPlayerBP) (Utilities|Struct|MakeBPS_DamageInfo (Math|Conversions|ToFloat(Integer) (Variables|Default|GetDamage%20Amount)) "NewEnumerator4" "NewEnumerator7" "NewEnumerator2")))

(event EventBeginPlay
  (Utilities|FlowControl|DoOnce false
    (:Completed
      (bind _returnvalue (Actor|GetActorOfClass "/Game/Assets/Blueprints/PlayerBP/PlayerCharacterBP.PlayerCharacterBP_C"))
      (Variables|Default|SetPlayerBP _returnvalue))))

(event EventTick
  (params (DeltaSeconds :type Float%20%28single-precision%29))
  (bind _playerbp (Variables|Default|GetPlayerBP))
  (bind _returnvalue (Transformation|GetActorLocation _playerbp))
  (Utilities|FlowControl|Delay 5.0)
  (Utilities|Time|SetTimerbyFunctionName 0 "" DeltaSeconds true)
  (if (not (AI|Components|NavMovement|IsFalling (Variables|/Script/Engine.Character|GetCharacterMovement (Variables|Default|GetPlayerBP))))
    (bind _outhit (Collision|LineTraceByChannel _returnvalue (+ _returnvalue "0.000000,0.000000,-100.000000") "TraceTypeQuery1" false 0 "None"))
    (Variables|Default|Setrespawn%20location (.location _outhit))))

(fn ConstructionScript)