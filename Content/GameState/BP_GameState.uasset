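; Game state Blueprint that owns the skill inventory screen for the RuneWarden player.
; On BeginPlay it caches the player pawn and creates the skill inventory widget once.
; The SkillInventory_UI event uses a FlipFlop to show or remove that widget, switching input mode, mouse cursor, pawn input and movement mode so the player is frozen while it is open.
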(event Custom|SkillInventory_UI
  (bind _returnvalue (Game|GetPlayerController 0))
  (bind _returnvalue_2 (Game|GetPlayerController 0))
  (Utilities|FlowControl|FlipFlop
    (:A
      (UserInterface|Viewport|AddtoViewport (Variables|Default|GetSkillInventory) 0)
      (Pawn|Components|CharacterMovement|SetMovementMode (Variables|/Script/Engine.Character|GetCharacterMovement (Variables|Default|GetPlayer_Ref)) "MOVE_None" 0)
      (Input|SetInputModeGameandUI _returnvalue (Variables|Default|GetSkillInventory) "DoNotLock" true false)
      (Variables|/Script/Engine.PlayerController|SetbShowMouseCursor _returnvalue true)
      (Input|DisableInput (Variables|Default|GetPlayer_Ref) (Game|GetPlayerController 0)))
    (:B
      (Widget|RemovefromParent (Variables|Default|GetSkillInventory))
      (Pawn|Components|CharacterMovement|SetMovementMode (Variables|/Script/Engine.Character|GetCharacterMovement (Variables|Default|GetPlayer_Ref)) "MOVE_Walking" 0)
      (Input|SetInputModeGameOnly _returnvalue_2 false)
      (Variables|/Script/Engine.PlayerController|SetbShowMouseCursor _returnvalue_2 false)
      (Input|EnableInput (Variables|Default|GetPlayer_Ref) (Game|GetPlayerController 0)))))

(event EventBeginPlay
  (bind _asplayer_character_bp (Utilities|Casting|CastToRuneWarden_BP (Game|Player|GetPlayerPawn 0)))
  (Variables|Default|SetPlayer_Ref _asplayer_character_bp)
  (bind _returnvalue (UserInterface|CreateWidget "/Game/Inventory/WBP_SkillInventory.WBP_SkillInventory_C" (Game|GetPlayerController 0)))
  (Variables|Default|SetSkillInventory _returnvalue))

(event EventTick
  (params (DeltaSeconds :type Float%20%28single-precision%29)))

(fn ConstructionScript)