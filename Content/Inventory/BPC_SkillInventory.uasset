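; Inventory component that tracks shard and scroll pickups and offers the player a choice of two random skills.
; Shard pickups trigger a GameInstance UI check at the max count, and scroll counts are stored on the GameInstance.
; SetSkillinfo draws two skills, removing them from the GameInstance's skill array, and shows them in WBP_SkillSelect.
; SkillUICheck maps each skill name to hardcoded description, aura background and icon.
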(event Custom|Set%20Skill%20info
  (bind _skillinventory (Variables|Default|GetSkillInventory))
  (bind _returnvalue (Utilities|Array|Length _skillinventory))
  (bind _returnvalue_2 (- _returnvalue 1))
  (bind _returnvalue_3 (Math|Random|RandomIntegerinRange 0 _returnvalue_2))
  (Utilities|FlowControl|Sequence
    (:then_0
      ;[1 0.662 0.8518] Set skill info to Skill 1
      (Variables|Default|SetSkillIndex1 _returnvalue_3)
      (Variables|Default|SetSKill1 (Utilities|Array|Get(acopy) (Variables|Default|GetSkillInventory) (Variables|Default|GetSkillIndex1)))
      (Utilities|Array|RemoveIndex (Variables|Default|GetSkillInventory) (Variables|Default|GetSkillIndex1))
      (Variables|/Game/GameState/BP_GameInstance.BP_GameInstance_C|SetSkillArray (Variables|Default|GetGame%20instance) (Variables|Default|GetSkillInventory))
      ;[0.01179 0.08912 1] Set Skill 1 info in UI
      (Variables|/Script/UMG.TextBlock|SetText (Variables|/Game/UI/WBP_SkillSelect.WBP_SkillSelect_C|GetSkillName1 (Variables|Default|GetWBP_SkillSelect)) (Utilities|Text|ToText(String) (Variables|Default|GetSKill1))))
    (:then_1
      ;[0.7651 0.5103 1] Set skill info for Skill 2
      (Variables|Default|SetSkillIndex2 _returnvalue_3)
      (Variables|Default|SetSkill2 (Utilities|Array|Get(acopy) (Variables|Default|GetSkillInventory) (Variables|Default|GetSkillIndex2)))
      (Utilities|Array|RemoveIndex (Variables|Default|GetSkillInventory) (Variables|Default|GetSkillIndex2))
      (Variables|/Game/GameState/BP_GameInstance.BP_GameInstance_C|SetSkillArray (Variables|Default|GetGame%20instance) (Variables|Default|GetSkillInventory))
      ;[0 0.06699 1] Set Skill 2 info in UI
      (Variables|/Script/UMG.TextBlock|SetText (Variables|/Game/UI/WBP_SkillSelect.WBP_SkillSelect_C|GetSkillName2 (Variables|Default|GetWBP_SkillSelect)) (Utilities|Text|ToText(String) (Variables|Default|GetSkill2)))))
  (CallFunction|SkillUICheck)
  ;[0.01923 0.02986 1] Open UI
  (UserInterface|Viewport|AddtoViewport (Variables|Default|GetWBP_SkillSelect) 0))

(event EventShardPickup
  ;[1 0 0.00169] Shard Pickup check against max shard count
  (bind _result (Math|Integer|IncrementInt (Variables|Default|GetShardCount))
    (:%20%20
      (bind _output_get (Variables|Default|SetShardCount _result))
      (if (== _output_get (Variables|Default|GetMaxShardCount))
        (Variables|Default|SetShardCount 0)
        (Default|ShardCheckUI (Variables|Default|GetGame%20instance))))))

(event EventBeginPlay
  ;[1 0.915 0] Begin Play Event
  (bind _returnvalue (UserInterface|CreateWidget "/Game/UI/WBP_SkillSelect.WBP_SkillSelect_C" (Game|GetPlayerController 0)))
  (Variables|Default|SetWBP_SkillSelect _returnvalue)
  (bind _asbp_game_instance (Utilities|Casting|CastToBP_GameInstance (Game|GetGameInstance)))
  (Variables|Default|SetGame%20instance _asbp_game_instance)
  (Variables|Default|SetSkillInventory (Variables|/Game/GameState/BP_GameInstance.BP_GameInstance_C|GetSkillArray _asbp_game_instance)))

(event EventScrollPickup
  (bind _result (Math|Integer|IncrementInt (Variables|Default|GetScroll%20Count))
    (:%20%20
      (bind _output_get (Variables|/Game/GameState/BP_GameInstance.BP_GameInstance_C|SetScroll%20Count (Variables|Default|GetGame%20instance) _result))
      (Development|PrintString (Utilities|String|ToString(Integer) _output_get)))))

(fn AddItemtoInventory
  (params (NewItem :type String%20%28by%20ref%29))
  (Utilities|Array|Add (Variables|Default|GetSkillInventory) NewItem)
  (Development|PrintString NewItem)
  (bind _asrune_warden_bp (Utilities|Casting|CastToRuneWarden_BP (Components|GetOwner)))
  (Default|AddItemtoListUI (Variables|/Game/Assets/Blueprints/PlayerBP/RuneWarden_BP.RuneWarden_BP_C|GetInventoryWidget _asrune_warden_bp) NewItem))

(fn SkillUICheck
  (bind _wbp_skillselect (Variables|Default|GetWBP_SkillSelect))
  (bind _wbp_skillselect_2 (Variables|Default|GetWBP_SkillSelect))
  (bind _skill1 (Variables|Default|GetSKill1))
  (bind _wbp_skillselect_3 (Variables|Default|GetWBP_SkillSelect))
  (bind _wbp_skillselect_4 (Variables|Default|GetWBP_SkillSelect))
  (bind _wbp_skillselect_5 (Variables|Default|GetWBP_SkillSelect))
  (bind _left_blue_aura (Variables|Default|GetLeft%20Blue%20Aura))
  (bind _left_red_aura (Variables|Default|GetLeft%20Red%20Aura))
  (bind _left_yellow_aura (Variables|Default|GetLeft%20Yellow%20Aura))
  (bind _left_green_aura (Variables|Default|GetLeft%20Green%20Aura))
  (bind _skill2 (Variables|Default|GetSkill2))
  (bind _wbp_skillselect_6 (Variables|Default|GetWBP_SkillSelect))
  (bind _right_blue_aura (Variables|Default|GetRight%20Blue%20Aura))
  (bind _right_red_aura (Variables|Default|GetRight%20Red%20Aura))
  (bind _right_yellow_aura (Variables|Default|GetRight%20Yellow%20Aura))
  (bind _right_green_aura (Variables|Default|GetRight%20Green%20Aura))
  (bind _skill1_description (Variables|/Game/UI/WBP_SkillSelect.WBP_SkillSelect_C|GetSkill1_Description _wbp_skillselect_3))
  (bind _leftside_image (Variables|/Game/UI/WBP_SkillSelect.WBP_SkillSelect_C|GetLeftSide_Image _wbp_skillselect_4))
  (bind _leftsideicon (Variables|/Game/UI/WBP_SkillSelect.WBP_SkillSelect_C|GetLeftSideIcon _wbp_skillselect_5))
  (bind _skill2_description (Variables|/Game/UI/WBP_SkillSelect.WBP_SkillSelect_C|GetSkill2_Description _wbp_skillselect_2))
  (bind _rightside_image (Variables|/Game/UI/WBP_SkillSelect.WBP_SkillSelect_C|GetRightSide_Image _wbp_skillselect))
  (bind _rightsideicon (Variables|/Game/UI/WBP_SkillSelect.WBP_SkillSelect_C|GetRightSideIcon _wbp_skillselect_6))
  (Utilities|FlowControl|Sequence
    (:then_0
      ;[0.15 0.15 0.15 0.5] Calm Aura
      (if (Utilities|Enum|Equal(Enum) _skill1 "Flurry Kicks")
        ;[0.15 0.15 0.15 0.5] Calm Aura
        (Variables|/Script/UMG.TextBlock|SetText _skill1_description "DropKick a Motha")
        ;[0.15 0.15 0.15 0.5] Set BackGround
        (Appearance|SetBrushfromTexture _leftside_image _left_blue_aura)
        ;[0.15 0.15 0.15 0.5] Set Icon for SKill
        (Appearance|SetBrushfromTexture _leftsideicon "/Game/Assets/Textures/Icons_UI/Light_FlurryKicks.Light_FlurryKicks")))
    (:then_1
      ;[0.15 0.15 0.15 0.5] Rage Aura
      (if (Utilities|Enum|Equal(Enum) _skill1 "Wicked Blows")
        ;[0.15 0.15 0.15 0.5] Rage Aura
        (Variables|/Script/UMG.TextBlock|SetText _skill1_description "Chuck Norris")
        (Appearance|SetBrushfromTexture _leftside_image _left_red_aura)
        (Appearance|SetBrushfromTexture _leftsideicon "/Game/Assets/Textures/Icons_UI/Light_WickedBlows.Light_WickedBlows")))
    (:then_2
      ;[0.15 0.15 0.15 0.5] Seize Aura
      (if (Utilities|Enum|Equal(Enum) _skill1 "Chain Link")
        ;[0.15 0.15 0.15 0.5] Seize Aura
        (Variables|/Script/UMG.TextBlock|SetText _skill1_description "UFC")
        (Appearance|SetBrushfromTexture _leftside_image _left_yellow_aura)
        (Appearance|SetBrushfromTexture _leftsideicon "/Game/Assets/Textures/Icons_UI/Light_ChainLinks.Light_ChainLinks")))
    (:then_3
      ;[0.15 0.15 0.15 0.5] Trickster Aura
      (if (Utilities|Enum|Equal(Enum) _skill1 "Feint")
        ;[0.15 0.15 0.15 0.5] Trickster Aura
        (Variables|/Script/UMG.TextBlock|SetText _skill1_description "Zelda Is a pal")
        (Appearance|SetBrushfromTexture _leftside_image _left_green_aura)
        (Appearance|SetBrushfromTexture _leftsideicon "/Game/Assets/Textures/Icons_UI/Light_Feint.Light_Feint")))
    (:then_4
      (if (Utilities|Enum|Equal(Enum) _skill1 "Bestial Slashes")
        (Variables|/Script/UMG.TextBlock|SetText _skill1_description "Link is a Buddy")
        (Appearance|SetBrushfromTexture _leftside_image _left_red_aura)
        (Appearance|SetBrushfromTexture _leftsideicon "/Game/Assets/Textures/Icons_UI/Heavy1_BestialSlashes.Heavy1_BestialSlashes")))
    (:then_5
      (if (Utilities|Enum|Equal(Enum) _skill1 "Palm Strike")
        (Variables|/Script/UMG.TextBlock|SetText _skill1_description "Rocket Launcher")
        (Appearance|SetBrushfromTexture _leftside_image _left_blue_aura)
        (Appearance|SetBrushfromTexture _leftsideicon "/Game/Assets/Textures/Icons_UI/Heavy_PalmStrike.Heavy_PalmStrike")))
    (:then_6
      (if (Utilities|Enum|Equal(Enum) _skill1 "Chain Lunge")
        (Variables|/Script/UMG.TextBlock|SetText _skill1_description "I am the DragonBorn")
        (Appearance|SetBrushfromTexture _leftside_image _left_yellow_aura)
        (Appearance|SetBrushfromTexture _leftsideicon "/Game/Assets/Textures/Icons_UI/Heavy_ChainLunge.Heavy_ChainLunge")))
    (:then_7
      (if (Utilities|Enum|Equal(Enum) _skill1 "Shooting Star")
        (Variables|/Script/UMG.TextBlock|SetText _skill1_description "Luigi is my Bro")
        (Appearance|SetBrushfromTexture _leftside_image _left_green_aura)
        (Appearance|SetBrushfromTexture _leftsideicon "/Game/Assets/Textures/Icons_UI/THeavy_ShootingStar.THeavy_ShootingStar")))
    (:then_8
      (if (Utilities|Enum|Equal(Enum) _skill1 "Spirit Bow")
        (Variables|/Script/UMG.TextBlock|SetText _skill1_description "Mario is better than me")
        (Appearance|SetBrushfromTexture _leftside_image _left_blue_aura)
        (Appearance|SetBrushfromTexture _leftsideicon "/Game/Assets/Textures/Icons_UI/Special_SpiritBow.Special_SpiritBow")))
    (:then_9
      (if (Utilities|Enum|Equal(Enum) _skill1 "Howl")
        (Variables|/Script/UMG.TextBlock|SetText _skill1_description "Im jealous of mario")
        (Appearance|SetBrushfromTexture _leftside_image _left_red_aura)
        (Appearance|SetBrushfromTexture _leftsideicon "/Game/Assets/Textures/Icons_UI/Special_Howl.Special_Howl")))
    (:then_10
      (if (Utilities|Enum|Equal(Enum) _skill1 "Capturing Field")
        (Variables|/Script/UMG.TextBlock|SetText _skill1_description "Indiana jones hates snakes")
        (Appearance|SetBrushfromTexture _leftside_image _left_yellow_aura)
        (Appearance|SetBrushfromTexture _leftsideicon "/Game/Assets/Textures/Icons_UI/Special_CapturingField.Special_CapturingField")))
    (:then_11
      (if (Utilities|Enum|Equal(Enum) _skill1 "Decoy")
        (Variables|/Script/UMG.TextBlock|SetText _skill1_description "Game of Thrones")
        (Appearance|SetBrushfromTexture _leftside_image _left_green_aura)
        (Appearance|SetBrushfromTexture _leftsideicon "/Game/Assets/Textures/Icons_UI/Special_Decoy.Special_Decoy")))
    (:then_12
      ;[0.15 0.15 0.15 0.5] Calm Aura
      (if (Utilities|Enum|Equal(Enum) _skill2 "Flurry Kicks")
        ;[0.15 0.15 0.15 0.5] Calm Aura
        (Variables|/Script/UMG.TextBlock|SetText _skill2_description "DropKick a Motha")
        ;[0.15 0.15 0.15 0.5] Set BackGround
        (Appearance|SetBrushfromTexture _rightside_image _right_blue_aura)
        ;[0.15 0.15 0.15 0.5] Set Icon for SKill
        (Appearance|SetBrushfromTexture _rightsideicon "/Game/Assets/Textures/Icons_UI/Light_FlurryKicks.Light_FlurryKicks")))
    (:then_13
      (if (Utilities|Enum|Equal(Enum) _skill2 "Palm Strike")
        (Variables|/Script/UMG.TextBlock|SetText _skill2_description "Rocket Launcher")
        (Appearance|SetBrushfromTexture _rightside_image _right_blue_aura)
        (Appearance|SetBrushfromTexture _rightsideicon "/Game/Assets/Textures/Icons_UI/Heavy_PalmStrike.Heavy_PalmStrike")))
    (:then_14
      (if (Utilities|Enum|Equal(Enum) _skill2 "Spirit Bow")
        (Variables|/Script/UMG.TextBlock|SetText _skill2_description "Mario is better than me")
        (Appearance|SetBrushfromTexture _rightside_image _right_blue_aura)
        (Appearance|SetBrushfromTexture _rightsideicon "/Game/Assets/Textures/Icons_UI/Special_SpiritBow.Special_SpiritBow")))
    (:then_15
      ;[0.15 0.15 0.15 0.5] Rage Aura
      (if (Utilities|Enum|Equal(Enum) _skill2 "Wicked Blows")
        ;[0.15 0.15 0.15 0.5] Rage Aura
        (Variables|/Script/UMG.TextBlock|SetText _skill2_description "Chuck Norris")
        (Appearance|SetBrushfromTexture _rightside_image _right_red_aura)
        (Appearance|SetBrushfromTexture _rightsideicon "/Game/Assets/Textures/Icons_UI/Light_WickedBlows.Light_WickedBlows")))
    (:then_16
      (if (Utilities|Enum|Equal(Enum) _skill2 "Bestial Slashes")
        (Variables|/Script/UMG.TextBlock|SetText _skill2_description "Link is a Buddy")
        (Appearance|SetBrushfromTexture _rightside_image _right_red_aura)
        (Appearance|SetBrushfromTexture _rightsideicon "/Game/Assets/Textures/Icons_UI/Heavy1_BestialSlashes.Heavy1_BestialSlashes")))
    (:then_17
      (if (Utilities|Enum|Equal(Enum) _skill2 "Howl")
        (Variables|/Script/UMG.TextBlock|SetText _skill2_description "Im jealous of mario")
        (Appearance|SetBrushfromTexture _rightside_image _right_red_aura)
        (Appearance|SetBrushfromTexture _rightsideicon "/Game/Assets/Textures/Icons_UI/Special_Howl.Special_Howl")))
    (:then_18
      ;[0.15 0.15 0.15 0.5] Seize Aura
      (if (Utilities|Enum|Equal(Enum) _skill2 "Chain Link")
        ;[0.15 0.15 0.15 0.5] Seize Aura
        (Variables|/Script/UMG.TextBlock|SetText _skill2_description "UFC")
        (Appearance|SetBrushfromTexture _rightside_image _right_yellow_aura)
        (Appearance|SetBrushfromTexture _rightsideicon "/Game/Assets/Textures/Icons_UI/Light_ChainLinks.Light_ChainLinks")))
    (:then_19
      (if (Utilities|Enum|Equal(Enum) _skill2 "Chain Lunge")
        (Variables|/Script/UMG.TextBlock|SetText _skill2_description "I am the DragonBorn")
        (Appearance|SetBrushfromTexture _rightside_image _right_yellow_aura)
        (Appearance|SetBrushfromTexture _rightsideicon "/Game/Assets/Textures/Icons_UI/Heavy_ChainLunge.Heavy_ChainLunge")))
    (:then_20
      (if (Utilities|Enum|Equal(Enum) _skill2 "Capturing Field")
        (Variables|/Script/UMG.TextBlock|SetText _skill2_description "Indiana jones hates snakes")
        (Appearance|SetBrushfromTexture _rightside_image _right_yellow_aura)
        (Appearance|SetBrushfromTexture _rightsideicon "/Game/Assets/Textures/Icons_UI/Special_CapturingField.Special_CapturingField")))
    (:then_21
      ;[0.15 0.15 0.15 0.5] Trickster Aura
      (if (Utilities|Enum|Equal(Enum) _skill2 "Feint")
        ;[0.15 0.15 0.15 0.5] Trickster Aura
        (Variables|/Script/UMG.TextBlock|SetText _skill2_description "Zelda Is a pal")
        (Appearance|SetBrushfromTexture _rightside_image _right_green_aura)
        (Appearance|SetBrushfromTexture _rightsideicon "/Game/Assets/Textures/Icons_UI/Light_Feint.Light_Feint")))
    (:then_22
      (if (Utilities|Enum|Equal(Enum) _skill2 "Shooting Star")
        (Variables|/Script/UMG.TextBlock|SetText _skill2_description "Luigi is my Bro")
        (Appearance|SetBrushfromTexture _rightside_image _right_green_aura)
        (Appearance|SetBrushfromTexture _rightsideicon "/Game/Assets/Textures/Icons_UI/THeavy_ShootingStar.THeavy_ShootingStar")))
    (:then_23
      (if (Utilities|Enum|Equal(Enum) _skill2 "Decoy")
        (Variables|/Script/UMG.TextBlock|SetText _skill2_description "Game of Thrones")
        (Appearance|SetBrushfromTexture _rightside_image _right_green_aura)
        (Appearance|SetBrushfromTexture _rightsideicon "/Game/Assets/Textures/Icons_UI/Special_Decoy.Special_Decoy")))))

(fn PickUpItem
  (return ""))